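; BP_SpeedZone is a trigger zone that sets the speed of AI vehicles entering its box.
; On overlap, an AI_VehicleCamera actor gets its StartSpeed set to the zone's Limit.
; Its OpenDRIVE_RoadControl AI controller then receives a TargetSpeed of Limit plus a small random offset, so vehicles vary above the limit.
; A zero Limit skips the offset, giving a target speed of zero.
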(event `self.Box.OnComponentBeginOverlap`
  (params (OverlappedComponent :type "PrimitiveComponent Object Reference") (OtherActor :type "Actor Object Reference") (OtherComp :type "PrimitiveComponent Object Reference") (OtherBodyIndex :type Integer) (bFromSweep :type Boolean) (SweepResult :type "HitResult Structure (by ref)"))
  (bind _limit (`self.Limit`))
  (bind _returnvalue (`KismetMathLibrary.Conv_IntToDouble` _limit))
  (bind _asai_vehicle_camera (cast `/EG4U/AI_VehicleCamera` OtherActor))
  (set `/EG4U/AI_VehicleCamera.StartSpeed` _returnvalue _asai_vehicle_camera)
  (bind _asopen_drive_road_control (cast `/EG4U/Vehicle/OpenDRIVE_RoadControl` (`AIBlueprintHelperLibrary.GetAIController` _asai_vehicle_camera)))
  (set `/EG4U/Vehicle/OpenDRIVE_RoadControl.TargetSpeed` (+ _returnvalue (`KismetMathLibrary.SelectFloat` 0.0 (`KismetMathLibrary.RandomFloatInRange` 2.0 12.0) (== _limit 0))) _asopen_drive_road_control))

(fn `UserConstructionScript`)