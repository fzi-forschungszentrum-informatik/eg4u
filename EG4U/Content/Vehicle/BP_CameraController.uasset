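; Camera director that switches the player's view between drone and stationary cameras in the level and picks which wheeled vehicle they track.
; BeginPlay collects both camera types and passes them ActorToTrack, then number keys blend to a camera by index.
; Up/Down cycle the tracked vehicle, re-appending every camera to the list each time.
; F toggles between viewing the current vehicle directly and the first camera.
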(event `Key|One`
  (params (Key :type "Key Structure"))
  (:`Pressed`
    (`self.MakeActiveCamera` 0)))

(event `self.ReceiveBeginPlay`
  (bind _actor_to_track (`self.Actor to Track`))
  (`|ExecutionSequence`
    (:`then_0`
      (bind _outactors (`GameplayStatics.GetAllActorsOfClass` "/EG4U/Vehicle/BP_CameraDrone.BP_CameraDrone_C"))
      (bind _outactors_2 (`GameplayStatics.GetAllActorsOfClass` "/EG4U/Vehicle/BP_CameraStationary.BP_CameraStationary_C"))
      (for _array_element _outactors
        (`KismetArrayLibrary.Array_Add` (`self.CameraComponents`) (`self.GetComponentByClass` _array_element "/Script/Engine.CameraComponent"))
        (set `/EG4U/Vehicle/BP_CameraDrone.Actor To Track` _actor_to_track _array_element))
      (for _array_element_2 _outactors_2
        (`KismetArrayLibrary.Array_Add` (`self.CameraComponents`) (`self.GetComponentByClass` _array_element_2 "/Script/Engine.CameraComponent"))
        (set `/EG4U/Vehicle/BP_CameraStationary.Actor To Track` _actor_to_track _array_element_2))
      (`self.MakeActiveCamera` 0))
    (:`then_1`
      (bind _outactors_3 (`GameplayStatics.GetAllActorsOfClass` "/Script/PhysXVehicles.WheeledVehicle"))
      (bind _output_get (set `self.Vehicles` _outactors_3))
      (bind _aswheeled_vehicle (cast `WheeledVehicle` (`|ConvertAsset` (`self.Actor to Track`))))
      (set `self.CurrentIndex` (`KismetArrayLibrary.Array_Find` _output_get _aswheeled_vehicle)))))

(event `Key|Two`
  (params (Key :type "Key Structure"))
  (:`Pressed`
    (`self.MakeActiveCamera` 1)))

(event `Key|Three`
  (params (Key :type "Key Structure"))
  (:`Pressed`
    (`self.MakeActiveCamera` 2)))

(event `Key|Four`
  (params (Key :type "Key Structure"))
  (:`Pressed`
    (`self.MakeActiveCamera` 3)))

(event `Key|Five`
  (params (Key :type "Key Structure"))
  (:`Pressed`
    (`self.MakeActiveCamera` 4)))

(event `MakeActiveCamera`
  (params (Index :type Integer))
  (if (<= Index (`KismetArrayLibrary.Array_LastIndex` (`self.CameraComponents`)))
    (for (_array_element _array_index) (`self.CameraComponents`)
      (if (== _array_index Index)
        (`ActorComponent.SetActive` _array_element true false)
        (`PlayerController.SetViewTargetWithBlend` (`GameplayStatics.GetPlayerController` 0) (`ActorComponent.GetOwner` _array_element) (`self.Blend Time`) "VTBlend_Linear" (`self.Blend Exp`) false)
        (else
          (`ActorComponent.SetActive` _array_element true false))))))

(event `Key|Six`
  (params (Key :type "Key Structure"))
  (:`Pressed`
    (`self.MakeActiveCamera` 5)))

(event `Key|Seven`
  (params (Key :type "Key Structure"))
  (:`Pressed`
    (`self.MakeActiveCamera` 6)))

(event `Key|Eight`
  (params (Key :type "Key Structure"))
  (:`Pressed`
    (`self.MakeActiveCamera` 7)))

(event `Key|Nine`
  (params (Key :type "Key Structure"))
  (:`Pressed`
    (`self.MakeActiveCamera` 8)))

(event `Key|F`
  (params (Key :type "Key Structure"))
  (:`Pressed`
    (`/Engine/EditorBlueprintResources/StandardMacros.FlipFlop`
      (:`A`
        (`PlayerController.SetViewTargetWithBlend` (`GameplayStatics.GetPlayerController` 0) (`|GetArrayItem` (`self.Vehicles`) (`self.CurrentIndex`)) (`self.Blend Time`) "VTBlend_Linear" (`self.Blend Exp`) false))
      (:`B`
        (`self.MakeActiveCamera` 0)))))

(event `Key|Zero`
  (params (Key :type "Key Structure"))
  (:`Pressed`
    (`self.MakeActiveCamera` 9)))

(event `Key|Down`
  (params (Key :type "Key Structure"))
  (bind _actor_to_track (`self.Actor to Track`))
  (bind _output (`|GetArrayItem` (`self.Vehicles`) (`self.CurrentIndex`)))
  (:`Pressed`
    (if (> (`self.CurrentIndex`) 0)
      (`/Engine/EditorBlueprintResources/StandardMacros.DecrementInt` (`self.CurrentIndex`)
        (:`  `
          _))
      (else
        (set `self.CurrentIndex` (`KismetArrayLibrary.Array_LastIndex` (`self.Vehicles`)))))
    (set `self.Actor to Track` (`|ConvertAsset` _output) :!label _label)
    (bind _outactors (`GameplayStatics.GetAllActorsOfClass` "/EG4U/Vehicle/BP_CameraDrone.BP_CameraDrone_C"))
    (bind _outactors_2 (`GameplayStatics.GetAllActorsOfClass` "/EG4U/Vehicle/BP_CameraStationary.BP_CameraStationary_C"))
    (for _array_element _outactors
      (`KismetArrayLibrary.Array_Add` (`self.CameraComponents`) (`self.GetComponentByClass` _array_element "/Script/Engine.CameraComponent"))
      (set `/EG4U/Vehicle/BP_CameraDrone.Actor To Track` _actor_to_track _array_element))
    (for _array_element_2 _outactors_2
      (`KismetArrayLibrary.Array_Add` (`self.CameraComponents`) (`self.GetComponentByClass` _array_element_2 "/Script/Engine.CameraComponent"))
      (set `/EG4U/Vehicle/BP_CameraStationary.Actor To Track` _actor_to_track _array_element_2))
    (`KismetSystemLibrary.PrintString` (`KismetStringLibrary.Concat_StrStr` "Camera: Focus on " (`KismetSystemLibrary.GetDisplayName` _output)) true true (struct :`G` 1.0 :`A` 1.0))))

(event `Key|Up`
  (params (Key :type "Key Structure"))
  (:`Pressed`
    (if (< (`self.CurrentIndex`) (`KismetArrayLibrary.Array_LastIndex` (`self.Vehicles`)))
      (`/Engine/EditorBlueprintResources/StandardMacros.IncrementInt` (`self.CurrentIndex`)
        (:`  `
          (goto _label)))
      (else
        (set `self.CurrentIndex` 0)
        (goto _label)))))

(fn `UserConstructionScript`)