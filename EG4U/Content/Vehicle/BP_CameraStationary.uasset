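; Stationary camera in the Vehicle folder that tracks a target actor (ActorToTrack) from a fixed position and zooms with distance.
; Each tick, a look-at aims the Joint component at the target using pitch and yaw, and clamped distance sets focal length between MinFocalLength and MaxFocalLength.
; The construction script sets an initial distance-based field of view, or prints a warning if the target is invalid.
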(event `self.ReceiveTick`
  (params (DeltaSeconds :type "Float (single-precision)"))
  (bind _returnvalue (`KismetAnimationLibrary.K2_LookAt` (`SceneComponent.K2_GetComponentToWorld` (`self.Joint`)) (`self.Target Position`) (10.0 0.0 0.0)))
  (set `self.Target Position` (`self.K2_GetActorLocation` (`|ConvertAsset` (`self.Actor To Track`))))
  (`SceneComponent.K2_SetWorldTransform` (`self.Joint`) (`KismetMathLibrary.MakeTransform` (.location _returnvalue) (`KismetMathLibrary.MakeRotator` 0.0 (.pitch (.rotation _returnvalue)) (.yaw (.rotation _returnvalue))) (.scale _returnvalue)) false false)
  (set `CineCameraComponent.CurrentFocalLength` (`KismetMathLibrary.MapRangeClamped` (`KismetMathLibrary.Vector_Distance` (`self.K2_GetActorLocation`) (`self.Target Position`)) 1000.0 15000.0 (`self.MinFocalLength`) (`self.MaxFocalLength`)) (`self.CameraComponent`)))

(fn `UserConstructionScript`
  (bind _output (`|ConvertAsset` (`self.Actor To Track`)))
  (if (`KismetSystemLibrary.IsValid` _output)
    (`CameraComponent.SetFieldOfView` (`self.CameraComponent`) (`KismetMathLibrary.MapRangeClamped` (`KismetMathLibrary.Vector_Distance` (`self.K2_GetActorLocation`) (`self.K2_GetActorLocation` _output)) 1000.0 10000.0 110.0 1.0))
    (else
      (`KismetSystemLibrary.PrintString` "Warning: Camera Target invalid"))))