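; Procedural building actor that builds a multi-storey building from a footprint, floor properties and OSM tags.
; It stacks attached BP_Procedural_Floor actors, accumulating height, with a distinct ground floor and a final roof-ledge floor on top.
; ConstructRoof, also run on construction, asks ParentGenerator for flat roof geometry from the footprint and an offset polygon, filling two procedural mesh sections.
; Regenerate clears the spawned floors and roof, then rebuilds from stored settings.
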(fn `AddOffsetToFootprint`
  (params (In :type "Array of Vector Structure") (Offset :type "Vector Structure"))
  (returns (Out :type "Array of Vector Structure"))
  (for _array_element In
    (`KismetArrayLibrary.Array_Add` (`self.Transformed`) (+ _array_element Offset)))
  (return (`self.Transformed`)))

(fn `ConstructBuilding`
  (params (Floors :type Integer) (Footprint :type "Array of Vector Structure") (GroundFloor :type "/EG4U/Data/LevelProperties Structure") (Facade :type "/EG4U/Data/LevelProperties Structure") (Reverse :type Boolean) (FakeWindows :type Boolean) (ID :type Integer) (`Osm Tags` :type "Map of String to String") (`Facade Material` :type "MaterialInterface Object Reference"))
  (set `self.Floors` Floors)
  (set `self.Footprint` Footprint)
  (set `self.Ground Floor` GroundFloor)
  (set `self.Facade` Facade)
  (set `self.Reverse` Reverse)
  (set `self.Fake Windows` FakeWindows)
  (set `self.Building Height` 0.0)
  (set `self.Building ID` ID)
  (set `self.Osm Tags` `Osm Tags`)
  (set `self.Facade Material` `Facade Material`)
  (`self.RemoveRoof`)
  (for _index (range (+ (`self.Floors`) 1))
    (`|ExecutionSequence`
      (:`then_0`
        (bind _returnvalue (`|SpawnActorFromClass` "/Game/DE/ProceduralGeneration/BP_Procedural_Floor.BP_Procedural_Floor_C" (`KismetMathLibrary.MakeTransform` (0.0 0.0 0.0)) "AlwaysSpawn" "OverrideRootScale" null null))
        (`/Game/DE/ProceduralGeneration/BP_Procedural_Floor.SetFootprint` _returnvalue (`local.Footprint`) (`self.Building Height`) (`self.Reverse`))
        (set `/Game/DE/ProceduralGeneration/BP_Procedural_Floor.Facade_Material` (`self.Facade Material`) _returnvalue)
        (`KismetArrayLibrary.Array_Add` (`self.Refs`) _returnvalue))
      (:`then_1`
        ;[1 1 1] Ground Floor
        (if (== _index 0)
          (set `/Game/DE/ProceduralGeneration/BP_Procedural_Floor.Properties` (`self.Ground Floor`) _returnvalue)
          (else
            (set `/Game/DE/ProceduralGeneration/BP_Procedural_Floor.Properties` (`self.Facade`) _returnvalue)))
        (set `/Game/DE/ProceduralGeneration/BP_Procedural_Floor.WindowBackdrop` (`self.Fake Windows`) _returnvalue))
      (:`then_2`
        (bind _height (`/Game/DE/ProceduralGeneration/BP_Procedural_Floor.GetFloorHeight` _returnvalue))
        (set `self.Building Height` (+ _height (`self.Building Height`)))
        (set `/Game/DE/ProceduralGeneration/BP_Procedural_Floor.LiveUpdate` true _returnvalue)
        (`/Game/DE/ProceduralGeneration/BP_Procedural_Floor.GenerateFloor` _returnvalue)
        (`KismetArrayLibrary.Array_Clear` (`self.Transformed`))
        (`self.K2_AttachToActor` _returnvalue self "None" "KeepRelative" "KeepRelative" "KeepRelative" true))))
  (`self.ConstructRoof`)
  (`|ExecutionSequence`
    (:`then_0`
      (bind _returnvalue_2 (`|SpawnActorFromClass` "/Game/DE/ProceduralGeneration/BP_Procedural_Floor.BP_Procedural_Floor_C" (`KismetMathLibrary.MakeTransform` (0.0 0.0 0.0)) "AlwaysSpawn" "OverrideRootScale" null null))
      (`/Game/DE/ProceduralGeneration/BP_Procedural_Floor.SetFootprint` _returnvalue_2 (`local.Footprint`) (`self.Building Height`) (`self.Reverse`))
      (`KismetArrayLibrary.Array_Add` (`self.Refs`) _returnvalue_2))
    (:`then_1`
      (set `/Game/DE/ProceduralGeneration/BP_Procedural_Floor.Properties` (make `/EG4U/Data/LevelProperties` "/Game/ModernCityEnvironment01/Meshes/SM_MBuilding02_RoofLedge_A.SM_MBuilding02_RoofLedge_A" "0.000000,0.000000,0.000000|0.000000,0.000000,0.000000|1.000000,1.000000,1.000000" 3 "/Game/ModernCityEnvironment01/Meshes/SM_MBuilding02_RoofLedge_A.SM_MBuilding02_RoofLedge_A" "0.000000,0.000000,0.000000|0.000000,0.000000,0.000000|1.000000,1.000000,1.000000" false "/Game/ModernCityEnvironment01/Meshes/SM_MBuilding02_RoofLedge_A.SM_MBuilding02_RoofLedge_A") _returnvalue_2)
      (set `/Game/DE/ProceduralGeneration/BP_Procedural_Floor.WindowBackdrop` (`self.Fake Windows`) _returnvalue_2))
    (:`then_2`
      (bind _height_2 (`/Game/DE/ProceduralGeneration/BP_Procedural_Floor.GetFloorHeight` _returnvalue_2))
      (set `/Game/DE/ProceduralGeneration/BP_Procedural_Floor.LiveUpdate` true _returnvalue_2)
      (`/Game/DE/ProceduralGeneration/BP_Procedural_Floor.GenerateFloor` _returnvalue_2)
      (`KismetArrayLibrary.Array_Clear` (`self.Transformed`))
      (`self.K2_AttachToActor` _returnvalue_2 self "None" "KeepRelative" "KeepRelative" "KeepRelative" true))))

(fn `ConstructRoof`
  (bind _building_height (`self.Building Height`))
  (bind _roof_height (`self.Roof Height`))
  (`|ExecutionSequence`
    (:`then_0`
      (`self.RemoveRoof`)
      (bind _returnvalue (`AddComponent|NODE_AddProceduralMeshComponent-0`))
      (set `self.RoofMesh` _returnvalue)
      (bind _returnvalue_2 (`OpenStreetMap_Generator.GenerateRoof` (`self.ParentGenerator`) (`self.Footprint`) (`self.Osm Tags`) "Flat" _building_height _roof_height))
      (`ProceduralMeshComponent.CreateMeshSection_LinearColor` :`self` (`self.RoofMesh`) :`Vertices` (break `OpenStreetMap_Generator_MeshInfo` _returnvalue_2) :`Triangles` (`.triangles` (break `OpenStreetMap_Generator_MeshInfo` _returnvalue_2)) :`UV0` (`.uv_coords` (break `OpenStreetMap_Generator_MeshInfo` _returnvalue_2)))
      (`PrimitiveComponent.SetMaterial` (`self.RoofMesh`) 0 (`self.RoofMaterial`))
      (bind _returnvalue_3 (`OpenStreetMap_Generator.OffsetPolygon` (`self.ParentGenerator`) (`self.Footprint`) (`self.Offset`) (+ _building_height _roof_height)))
      (bind _returnvalue_4 (`OpenStreetMap_Generator.GenerateRoof` (`self.ParentGenerator`) _returnvalue_3 (`self.Osm Tags`) "Flat" _building_height _roof_height))
      (`ProceduralMeshComponent.CreateMeshSection_LinearColor` :`self` (`self.RoofMesh`) :`SectionIndex` 1 :`Vertices` (break `OpenStreetMap_Generator_MeshInfo` _returnvalue_4) :`Triangles` (`.triangles` (break `OpenStreetMap_Generator_MeshInfo` _returnvalue_4)) :`UV0` (`.uv_coords` (break `OpenStreetMap_Generator_MeshInfo` _returnvalue_4)))
      (`PrimitiveComponent.SetMaterial` (`self.RoofMesh`) 1 "/Game/DE/Dev/Material/VISUALIZER/UV_TEST05.UV_TEST05"))))

(fn `Regenerate`
  (`self.RemoveBuilding`)
  (set `self.Building Height` 0.0)
  (for _index (range (+ (`self.Floors`) 1))
    (`|ExecutionSequence`
      (:`then_0`
        (bind _returnvalue (`|SpawnActorFromClass` "/Game/DE/ProceduralGeneration/BP_Procedural_Floor.BP_Procedural_Floor_C" (`KismetMathLibrary.MakeTransform` (0.0 0.0 0.0)) "AlwaysSpawn" "OverrideRootScale" null null))
        (`/Game/DE/ProceduralGeneration/BP_Procedural_Floor.SetFootprint` _returnvalue (`self.Footprint`) (`self.Building Height`) (`self.Reverse`))
        (`KismetArrayLibrary.Array_Add` (`self.Refs`) _returnvalue))
      (:`then_1`
        ;[1 1 1] Ground Floor
        (if (== _index 0)
          (set `/Game/DE/ProceduralGeneration/BP_Procedural_Floor.Properties` (`self.Ground Floor`) _returnvalue)
          (else
            (set `/Game/DE/ProceduralGeneration/BP_Procedural_Floor.Properties` (`self.Facade`) _returnvalue)))
        (set `/Game/DE/ProceduralGeneration/BP_Procedural_Floor.WindowBackdrop` (`self.Fake Windows`) _returnvalue))
      (:`then_2`
        ;[1 1 1] Roof
        (if (== _index 0)
          _))
      (:`then_3`
        (bind _height (`/Game/DE/ProceduralGeneration/BP_Procedural_Floor.GetFloorHeight` _returnvalue))
        (set `self.Building Height` (+ _height (`self.Building Height`)))
        (set `/Game/DE/ProceduralGeneration/BP_Procedural_Floor.LiveUpdate` true _returnvalue)
        (`/Game/DE/ProceduralGeneration/BP_Procedural_Floor.GenerateFloor` _returnvalue)
        (`KismetArrayLibrary.Array_Clear` (`self.Transformed`))
        (`self.K2_AttachToActor` _returnvalue self "None" "KeepRelative" "KeepRelative" "KeepRelative" true))))
  (`self.ConstructRoof`)
  (`|ExecutionSequence`
    (:`then_0`
      (bind _returnvalue_2 (`|SpawnActorFromClass` "/Game/DE/ProceduralGeneration/BP_Procedural_Floor.BP_Procedural_Floor_C" (`KismetMathLibrary.MakeTransform` (0.0 0.0 0.0)) "AlwaysSpawn" "OverrideRootScale" null null))
      (`/Game/DE/ProceduralGeneration/BP_Procedural_Floor.SetFootprint` _returnvalue_2 (`self.Footprint`) (`self.Building Height`) (`self.Reverse`))
      (set `/Game/DE/ProceduralGeneration/BP_Procedural_Floor.Facade_Material` (`self.Facade Material`) _returnvalue_2)
      (`KismetArrayLibrary.Array_Add` (`self.Refs`) _returnvalue_2))
    (:`then_1`
      (set `/Game/DE/ProceduralGeneration/BP_Procedural_Floor.Properties` (make `/EG4U/Data/LevelProperties` "/EG4U/Static/Mesh/SM_Roof_Ledge.SM_Roof_Ledge" "0.000000,0.000000,0.000000|0.000000,0.000000,0.000000|1.000000,1.000000,1.000000" 3 "/EG4U/Static/Mesh/SM_Roof_Ledge.SM_Roof_Ledge" "0.000000,0.000000,0.000000|0.000000,0.000000,0.000000|1.000000,1.000000,1.000000" false "/Game/ModernCityEnvironment01/Meshes/SM_MBuilding02_RoofLedge_A.SM_MBuilding02_RoofLedge_A") _returnvalue_2)
      (set `/Game/DE/ProceduralGeneration/BP_Procedural_Floor.WindowBackdrop` (`self.Fake Windows`) _returnvalue_2))
    (:`then_2`
      (bind _height_2 (`/Game/DE/ProceduralGeneration/BP_Procedural_Floor.GetFloorHeight` _returnvalue_2))
      (set `/Game/DE/ProceduralGeneration/BP_Procedural_Floor.LiveUpdate` true _returnvalue_2)
      (`/Game/DE/ProceduralGeneration/BP_Procedural_Floor.GenerateFloor` _returnvalue_2)
      (`KismetArrayLibrary.Array_Clear` (`self.Transformed`))
      (`self.K2_AttachToActor` _returnvalue_2 self "None" "KeepRelative" "KeepRelative" "KeepRelative" true))))

(fn `RemoveBuilding`
  (bind _refs (`self.Refs`))
  (for _array_element _refs
    (`/Game/DE/ProceduralGeneration/BP_Procedural_Floor.RemoveFloor` _array_element)
    (`self.K2_DestroyActor` _array_element))
  (`KismetArrayLibrary.Array_Clear` _refs)
  (`self.RemoveRoof`))

(fn `RemoveRoof`
  (bind _roofmesh (`self.RoofMesh`))
  (`ProceduralMeshComponent.ClearAllMeshSections` _roofmesh)
  (`ActorComponent.K2_DestroyComponent` _roofmesh))

(fn `UserConstructionScript`
  (`self.ConstructRoof`))