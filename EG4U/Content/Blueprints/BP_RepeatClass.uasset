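; BP_RepeatClass is a spline placement tool that repeats a chosen actor class at fixed spacing along its spline.
; The construction script destroys the tracked actors and, when LiveUpdate is on, calls SpawnObjects.
; SpawnObjects steps along the spline by Space, spawning at world-space points with a rotation offset added and recording each actor.
; RemoveObjects clears them; spawned actors stay unattached, as the attach node is unwired.
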(fn `RemoveObjects`
  (bind _actors (`self.Actors`))
  (for _array_element _actors
    (`self.K2_DestroyActor` _array_element))
  (`KismetArrayLibrary.Array_Clear` _actors))

(fn `SpawnObjects`
  (bind (_relative_transform_rotation_roll _relative_transform_rotation_pitch _relative_transform_rotation_yaw) (`KismetMathLibrary.BreakRotator` (`self.Relative Transform Rotation`)))
  (bind _returnvalue (`SplineComponent.GetTransformAtDistanceAlongSpline` (`self.Spline`) (`self.Current Length`) "World" false))
  (while (< (`self.Current Length`) (`SplineComponent.GetSplineLength` (`self.Spline`)))
    (bind _returnvalue_2 (`|SpawnActorFromClass` (`self.ObjectClass`) (`KismetMathLibrary.MakeTransform` (.location _returnvalue) (`KismetMathLibrary.MakeRotator` (+ _relative_transform_rotation_roll (.roll (.rotation _returnvalue))) (+ _relative_transform_rotation_pitch (.pitch (.rotation _returnvalue))) (+ _relative_transform_rotation_yaw (.yaw (.rotation _returnvalue))))) "Undefined" "OverrideRootScale" null null))
    (`KismetArrayLibrary.Array_Add` (`self.Actors`) _returnvalue_2)
    (set `self.Current Length` (+ (`self.Current Length`) (`self.Space`)))))

(fn `UserConstructionScript`
  (bind _actors (`self.Actors`))
  (for _array_element _actors
    (`self.K2_DestroyActor` _array_element))
  (`KismetArrayLibrary.Array_Clear` _actors)
  (if (`self.Live Update`)
    (`self.SpawnObjects`)))