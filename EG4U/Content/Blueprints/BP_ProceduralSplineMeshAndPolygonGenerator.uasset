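; Spline-driven generator that lays a mesh along a spline, with a custom-depth semantic stencil on its instanced mesh.
; Construction (LiveUpdate) or GenerateMeshes builds either deformed spline mesh components or straight instances.
; CalculateScale stretches pieces to fit each segment, or the whole spline under GenerateMeshes' SmartDistribution.
; GeneratePolygon samples the outline for MakePolygon, whose triangulation and procedural-mesh nodes are unreachable.
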(event `RemovePolygon`
  ;[1 0 0] Destructor
  (`self.ClearMeshes`))

(event `UpdateSplinePoints`
  (bind _shape (`self.Shape`))
  (bind (_returnvalue_x _returnvalue_y _returnvalue_z) (`KismetMathLibrary.BreakVector` (`SplineComponent.GetLocationAtDistanceAlongSpline` _shape 0.0 "Local")))
  (bind _returnvalue (select `bool` (`self.Curved`) :`false` (- (`SplineComponent.GetNumberOfSplinePoints` _shape) 1) :`true` (* (`self.Parts`) (`self.PolyResolution`))))
  ;[1 1 0] Point Update
  (for _index (range (+ _returnvalue 1))
    (bind (_returnvalue_x_2 _returnvalue_y_2 _returnvalue_z_2) (`KismetMathLibrary.BreakVector` (`SplineComponent.GetLocationAtDistanceAlongSpline` _shape (* _index (/ (`SplineComponent.GetSplineLength` _shape) (`KismetMathLibrary.Conv_IntToDouble` _returnvalue))) "Local")))
    (`KismetArrayLibrary.Array_Add` (`self.Points2D`) (`KismetMathLibrary.MakeVector2D` _returnvalue_x_2 _returnvalue_y_2))
    (`KismetArrayLibrary.Array_Add` (`self.X3`) _returnvalue_z_2)
    (`SplineComponent.SetSplinePointType` _shape _index (`self.SplineType`) true))
  (`KismetArrayLibrary.Array_Add` (`self.Points2D`) (`KismetMathLibrary.MakeVector2D` _returnvalue_x _returnvalue_y))
  (`KismetArrayLibrary.Array_Add` (`self.X3`) _returnvalue_z)
  (if true
    _))

(event `RemoveMeshes`
  ;[1 0 0] Destructor
  (`self.ClearComponents`))

(event `ComputeHeightProfile`
  (params (InPoints :type "Array of Vector Structure") (HeightProfile :type "Array of Float (double-precision)"))
  (set `self.SplineHeight` HeightProfile)
  (for _index (range (+ (`KismetArrayLibrary.Array_LastIndex` InPoints) 1))
    (`SplineComponent.AddPoint` (`self.Shape`) (make `SplinePoint` 0.0 (`|GetArrayItem` InPoints _index) (0.0 0.0 0.0) (0.0 0.0 0.0) (struct) (`KismetMathLibrary.MakeVector` 1.0 1.0 (`|GetArrayItem` HeightProfile _index)) "Linear") true)))

(event `GeneratePolygon`
  (bind _shape (`self.Shape`))
  (bind (_returnvalue_x _returnvalue_y _returnvalue_z) (`KismetMathLibrary.BreakVector` (`SplineComponent.GetLocationAtDistanceAlongSpline` _shape 0.0 "Local")))
  (bind _returnvalue (select `bool` (`self.Curved`) :`false` (- (`SplineComponent.GetNumberOfSplinePoints` _shape) 1) :`true` (* (`self.Parts`) (`self.PolyResolution`))))
  ;[1 0 1] Polygon Generation
  (for _index (range (+ _returnvalue 1))
    (bind (_returnvalue_x_2 _returnvalue_y_2 _returnvalue_z_2) (`KismetMathLibrary.BreakVector` (`SplineComponent.GetLocationAtDistanceAlongSpline` _shape (* _index (/ (`SplineComponent.GetSplineLength` _shape) (`KismetMathLibrary.Conv_IntToDouble` _returnvalue))) "Local")))
    (`KismetArrayLibrary.Array_Add` (`self.Points2D`) (`KismetMathLibrary.MakeVector2D` _returnvalue_x_2 _returnvalue_y_2))
    (`KismetArrayLibrary.Array_Add` (`self.X3`) _returnvalue_z_2)
    (`SplineComponent.SetSplinePointType` _shape _index (`self.SplineType`) true))
  (`KismetArrayLibrary.Array_Add` (`self.Points2D`) (`KismetMathLibrary.MakeVector2D` _returnvalue_x _returnvalue_y))
  (`KismetArrayLibrary.Array_Add` (`self.X3`) _returnvalue_z)
  (if (>= _index 2)
    (`self.Make Polygon` (`self.Points2D`) (`self.X3`) (`self.SurfaceOffset`))
    (if (`self.SaveProceduralSurface`)
      _)))

(event `GenerateMeshes`
  (bind _scale_x (`KismetMathLibrary.BreakVector` (`self.Scale`)))
  (bind (_scale_x_2 _scale_y _scale_z) (`KismetMathLibrary.BreakVector` (`self.Scale`)))
  (bind _tangentresolution (`self.TangentResolution`))
  (bind _shape (`self.Shape`))
  (bind _shape_2 (`self.Shape`))
  (bind (_scale_x_3 _scale_y_2 _scale_z_2) (`KismetMathLibrary.BreakVector` (`self.Scale`)))
  (bind _scale_x_4 (`KismetMathLibrary.BreakVector` (`self.Scale`)))
  (bind _shape_3 (`self.Shape`))
  (bind (_scale_x_5 _scale_y_3 _scale_z_3) (`KismetMathLibrary.BreakVector` (`self.Scale`)))
  (bind (_scale_x_6 _scale_y_4 _scale_z_4) (`KismetMathLibrary.BreakVector` (`self.Scale`)))
  (bind (_returnvalue_origin _returnvalue_boxextent) (`KismetMathLibrary.BreakBoxSphereBounds` (`StaticMesh.GetBounds` (`self.SplineMesh`))))
  (bind (_returnvalue_origin_2 _returnvalue_boxextent_2) (`KismetMathLibrary.BreakBoxSphereBounds` (`StaticMesh.GetBounds` (`self.SplineMesh`))))
  (bind _returnvalue (`SplineComponent.GetTransformAtDistanceAlongSpline` _shape_3 0.0 "World" true))
  (bind _returnvalue_2 (`SplineComponent.GetTransformAtDistanceAlongSpline` _shape_2 0.0 "World" true))
  (bind _returnvalue_x (`KismetMathLibrary.BreakVector` (* _returnvalue_boxextent _scale_x_4)))
  (bind _returnvalue_x_2 (`KismetMathLibrary.BreakVector` (* (* _returnvalue_boxextent_2 2) _scale_x)))
  ;[1 0.1366 0] Conventional Generation Method
  (`StaticMeshComponent.SetStaticMesh` (`self.Mesh`) (`self.SplineMesh`))
  (if (not (`self.StraightenMeshes`))
    (if (`self.SmartDistribution`)
      ;[0 1 0] Fetch Road Points and set Spline Points
      (bind (_scale _parts) (`self.CalculateScale` (`SplineComponent.GetSplineLength` (`self.Shape`)) _returnvalue_x))
      (for _index (range _parts)
        ;[0 1 0] Setup Spline Mesh Component based on Road Type
        (bind _returnvalue_3 (`AddComponent|NODE_AddSplineMeshComponent-1` :`bManualAttachment` true))
        (`StaticMeshComponent.SetStaticMesh` _returnvalue_3 (`self.SplineMesh`))
        ;[0 1 0] Finish Spline Mesh Component
        (if (> _index 0)
          (bind _returnvalue_4 (* _scale _returnvalue_x))
          (bind _returnvalue_5 (* _index _returnvalue_4))
          (bind _returnvalue_6 (`SplineComponent.GetTransformAtDistanceAlongSpline` _shape_3 _returnvalue_5 "World" true))
          (bind _returnvalue_7 (+ _returnvalue_5 _returnvalue_4))
          (bind _returnvalue_8 (`SplineComponent.GetTransformAtDistanceAlongSpline` _shape_3 _returnvalue_7 "World" false))
          (bind _returnvalue_9 (`KismetMathLibrary.TransformLocation` _returnvalue_8 (`self.Offset`)))
          (bind _returnvalue_10 (/ (`SplineComponent.GetTangentAtDistanceAlongSpline` _shape_3 _returnvalue_7 "World") _tangentresolution))
          (`SplineMeshComponent.SetStartAndEnd` _returnvalue_3 (`KismetMathLibrary.TransformLocation` _returnvalue_6 (`self.Offset`)) (/ (`SplineComponent.GetTangentAtDistanceAlongSpline` _shape_3 _returnvalue_5 "World") _tangentresolution) _returnvalue_9 _returnvalue_10 true)
          (if (`self.CustomScale`)
            (`SplineMeshComponent.SetStartScale` _returnvalue_3 (`KismetMathLibrary.MakeVector2D` _scale_y_2 _scale_z_2) true)
            (`SplineMeshComponent.SetEndScale` _returnvalue_3 (`KismetMathLibrary.MakeVector2D` _scale_y_2 _scale_z_2) true)
            (else
              (`SplineMeshComponent.SetStartScale` _returnvalue_3 (`KismetMathLibrary.MakeVector2D` (.y (.scale _returnvalue_6)) (.z (.scale _returnvalue_6))) true)
              (`SplineMeshComponent.SetEndScale` _returnvalue_3 (`KismetMathLibrary.MakeVector2D` (.y (.scale _returnvalue_8)) (.z (.scale _returnvalue_8))) true)))
          (else
            (`SplineMeshComponent.SetStartAndEnd` _returnvalue_3 (`KismetMathLibrary.TransformLocation` _returnvalue (`self.Offset`)) (0.0 0.0 0.0) _returnvalue_9 _returnvalue_10 true)
            (if (`self.CustomScale`)
              (`SplineMeshComponent.SetStartScale` _returnvalue_3 (`KismetMathLibrary.MakeVector2D` _scale_y_2 _scale_z_2) true)
              (`SplineMeshComponent.SetEndScale` _returnvalue_3 (`KismetMathLibrary.MakeVector2D` _scale_y_2 _scale_z_2) true)
              (else
                (`SplineMeshComponent.SetStartScale` _returnvalue_3 (`KismetMathLibrary.MakeVector2D` (.y (.scale _returnvalue)) (.z (.scale _returnvalue))) true)
                (`SplineMeshComponent.SetEndScale` _returnvalue_3 (`KismetMathLibrary.MakeVector2D` (.y (.scale _returnvalue_8)) (.z (.scale _returnvalue_8))) true)))))
        (`PrimitiveComponent.SetCollisionEnabled` _returnvalue_3 "QueryAndPhysics")
        (`KismetArrayLibrary.Array_Add` (`self.StaticComponents`) _returnvalue_3))
      (set `self.Parts` _parts)
      ;[0 0.5572 1] Close Spline Mesh
      (if (`self.Closed`)
        (bind _returnvalue_11 (`AddComponent|NODE_AddSplineMeshComponent-2` :`bManualAttachment` true))
        (`StaticMeshComponent.SetStaticMesh` _returnvalue_11 (`self.SplineMesh`))
        (bind _returnvalue_12 (+ _returnvalue_5 _returnvalue_4))
        (bind _returnvalue_13 (`SplineComponent.GetTransformAtDistanceAlongSpline` _shape_2 _returnvalue_12 "World" true))
        ;[0 0.5572 1] Finish Spline Mesh Component
        (`SplineMeshComponent.SetStartAndEnd` _returnvalue_11 (`KismetMathLibrary.TransformLocation` _returnvalue_13 (`self.Offset`)) (/ (`SplineComponent.GetTangentAtDistanceAlongSpline` _shape_2 _returnvalue_12 "World") (`self.TangentResolution`)) (`KismetMathLibrary.TransformLocation` _returnvalue_2 (`self.Offset`)) (0.0 0.0 0.0) true)
        (if (`self.CustomScale`)
          (`SplineMeshComponent.SetStartScale` _returnvalue_11 (`KismetMathLibrary.MakeVector2D` _scale_y_3 _scale_z_3) true)
          (`SplineMeshComponent.SetEndScale` _returnvalue_11 (`KismetMathLibrary.MakeVector2D` _scale_y_4 _scale_z_4) true)
          (else
            (`SplineMeshComponent.SetStartScale` _returnvalue_11 (`KismetMathLibrary.MakeVector2D` (.y (.scale _returnvalue_2)) (.z (.scale _returnvalue_13))) true)
            (`SplineMeshComponent.SetEndScale` _returnvalue_11 (`KismetMathLibrary.MakeVector2D` (.y (.scale _returnvalue_13)) (.z (.scale _returnvalue_2))) true)))
        (`PrimitiveComponent.SetCollisionEnabled` _returnvalue_11 "QueryAndPhysics")
        (`KismetArrayLibrary.Array_Add` (`self.StaticComponents`) _returnvalue_11))
      (else
        (for _index_2 (range (`SplineComponent.GetNumberOfSplinePoints` (`self.Shape`)))
          (`self.GenerateSplinePart` (`self.SurfaceOffset`) (`self.SplineMesh`) _index_2))))
    (else
      (for _index_3 (range (`SplineComponent.GetNumberOfSplinePoints` (`self.Shape`)))
        (bind _returnvalue_14 (`SplineComponent.GetDistanceAlongSplineAtSplinePoint` _shape _index_3))
        (bind (_scale_2 _parts_2) (`self.CalculateScale` (- (`SplineComponent.GetDistanceAlongSplineAtSplinePoint` _shape (+ _index_3 1)) _returnvalue_14) _returnvalue_x_2))
        (for _index_4 (range _parts_2)
          (bind (_returnvalue_location _returnvalue_rotation) (`KismetMathLibrary.BreakTransform` (`SplineComponent.GetTransformAtDistanceAlongSpline` (`self.Shape`) (+ (* _index_4 (* _scale_2 _returnvalue_x_2)) _returnvalue_14) "Local" true)))
          (`InstancedStaticMeshComponent.AddInstance` (`self.Mesh`) (`KismetMathLibrary.MakeTransform` _returnvalue_location _returnvalue_rotation (`KismetMathLibrary.MakeVector` (+ (- _scale_2 1.0) _scale_x_2) _scale_y _scale_z))))))))

(fn `CalculateScale`
  (params (SplineLength :type "Float (double-precision)") (MeshSize :type "Float (double-precision)"))
  (returns (Scale :type "Float (double-precision)") (Parts :type Integer))
  (bind (_remainder _returnvalue) (`KismetMathLibrary.FMod` SplineLength MeshSize))
  (bind _returnvalue_2 (/ _remainder MeshSize))
  (bind _returnvalue_3 (!= _returnvalue 0))
  (return (select `bool` _returnvalue_3 :`false` _returnvalue_2 :`true` (+ (/ _returnvalue_2 (`KismetMathLibrary.SelectFloat` (`KismetMathLibrary.Conv_IntToDouble` _returnvalue) 1.0 _returnvalue_3)) 1.0)) (select `bool` _returnvalue_3 :`false` 1 :`true` _returnvalue)))

(fn `ClearComponents`
  (bind _staticcomponents (`self.StaticComponents`))
  (for _array_element _staticcomponents
    (`ActorComponent.K2_DestroyComponent` _array_element))
  (`KismetArrayLibrary.Array_Clear` _staticcomponents))

(fn `ClearMeshes`
  (bind _proceduraltriangles (`self.ProceduralTriangles`))
  (for _array_element _proceduraltriangles
    (`ActorComponent.K2_DestroyComponent` _array_element))
  (`KismetArrayLibrary.Array_Clear` _proceduraltriangles))

(fn `GenerateSplinePart`
  (params (Height :type "Float (double-precision)") (InMesh :type "StaticMesh Object Reference") (PointIndex :type Integer))
  (bind (_returnvalue_origin _returnvalue_boxextent) (`KismetMathLibrary.BreakBoxSphereBounds` (`StaticMesh.GetBounds` InMesh)))
  (bind _scale_x (`KismetMathLibrary.BreakVector` (`self.Scale`)))
  (bind _shape (`self.Shape`))
  (bind _shape_2 (`self.Shape`))
  (bind _tangentresolution (`self.TangentResolution`))
  (bind (_scale_x_2 _scale_y _scale_z) (`KismetMathLibrary.BreakVector` (`self.Scale`)))
  (bind _returnvalue (`SplineComponent.GetDistanceAlongSplineAtSplinePoint` _shape PointIndex))
  (bind _returnvalue_x (`KismetMathLibrary.BreakVector` (* _returnvalue_boxextent (* 2 _scale_x))))
  (bind _returnvalue_2 (`SplineComponent.GetTransformAtDistanceAlongSpline` _shape_2 _returnvalue "World" true))
  ;[0 1 0] Fetch Points and set Spline Points
  (bind (_scale _parts) (`self.CalculateScale` (- (`SplineComponent.GetDistanceAlongSplineAtSplinePoint` _shape (+ PointIndex 1)) _returnvalue) _returnvalue_x))
  (for _index (range _parts)
    ;[0 1 0] Setup Spline Mesh Component based on Road Type
    (bind _returnvalue_3 (`AddComponent|NODE_AddSplineMeshComponent-7` :`bManualAttachment` true :`RelativeTransform` (`KismetMathLibrary.MakeTransform` (`KismetMathLibrary.MakeVector` 0.0 0.0 Height))))
    (`StaticMeshComponent.SetStaticMesh` _returnvalue_3 InMesh)
    ;[0 1 0] Finish Spline Mesh Component
    (if (> _index 0)
      (bind _returnvalue_4 (* _scale _returnvalue_x))
      (bind _returnvalue_5 (+ (* _index _returnvalue_4) _returnvalue))
      (bind _returnvalue_6 (`SplineComponent.GetTransformAtDistanceAlongSpline` _shape_2 _returnvalue_5 "World" true))
      (bind _returnvalue_7 (+ _returnvalue_5 _returnvalue_4))
      (bind _returnvalue_8 (`SplineComponent.GetTransformAtDistanceAlongSpline` _shape_2 _returnvalue_7 "World" false))
      (bind _returnvalue_9 (`KismetMathLibrary.TransformLocation` _returnvalue_8 (`self.Offset`)))
      (bind _returnvalue_10 (/ (`SplineComponent.GetTangentAtDistanceAlongSpline` _shape_2 _returnvalue_7 "World") _tangentresolution))
      (`SplineMeshComponent.SetStartAndEnd` _returnvalue_3 (`KismetMathLibrary.TransformLocation` _returnvalue_6 (`self.Offset`)) (/ (`SplineComponent.GetTangentAtDistanceAlongSpline` _shape_2 _returnvalue_5 "World") _tangentresolution) _returnvalue_9 _returnvalue_10 true)
      (if (`self.CustomScale`)
        (`SplineMeshComponent.SetStartScale` _returnvalue_3 (`KismetMathLibrary.MakeVector2D` _scale_y _scale_z) true)
        (`SplineMeshComponent.SetEndScale` _returnvalue_3 (`KismetMathLibrary.MakeVector2D` _scale_y _scale_z) true)
        (else
          (`SplineMeshComponent.SetStartScale` _returnvalue_3 (`KismetMathLibrary.MakeVector2D` (.y (.scale _returnvalue_6)) (.z (.scale _returnvalue_6))) true)
          (`SplineMeshComponent.SetEndScale` _returnvalue_3 (`KismetMathLibrary.MakeVector2D` (.y (.scale _returnvalue_8)) (.z (.scale _returnvalue_8))) true)))
      (else
        (`SplineMeshComponent.SetStartAndEnd` _returnvalue_3 (`KismetMathLibrary.TransformLocation` _returnvalue_2 (`self.Offset`)) (/ (`SplineComponent.GetTangentAtDistanceAlongSpline` _shape_2 _returnvalue "World") _tangentresolution) _returnvalue_9 _returnvalue_10 true)
        (if (`self.CustomScale`)
          (`SplineMeshComponent.SetStartScale` _returnvalue_3 (`KismetMathLibrary.MakeVector2D` _scale_y _scale_z) true)
          (`SplineMeshComponent.SetEndScale` _returnvalue_3 (`KismetMathLibrary.MakeVector2D` _scale_y _scale_z) true)
          (else
            (`SplineMeshComponent.SetStartScale` _returnvalue_3 (`KismetMathLibrary.MakeVector2D` (.y (.scale _returnvalue_2)) (.z (.scale _returnvalue_2))) true)
            (`SplineMeshComponent.SetEndScale` _returnvalue_3 (`KismetMathLibrary.MakeVector2D` (.y (.scale _returnvalue_8)) (.z (.scale _returnvalue_8))) true)))))
    (`PrimitiveComponent.SetCollisionEnabled` _returnvalue_3 "QueryAndPhysics")
    (`KismetArrayLibrary.Array_Add` (`self.StaticComponents`) _returnvalue_3))
  (set `self.Parts` _parts))

(fn `Make Polygon`
  (params (InPoints :type "Array of Vector2D Structure") (Z :type "Array of Float (double-precision)") (Height :type "Float (double-precision)"))
  (returns (NewParam :type "ProceduralMeshComponent Object Reference"))
  (`|ExecutionSequence`))

(fn `Update Point Type`
  (for _index (range (`SplineComponent.GetNumberOfSplinePoints` (`self.Shape`)))
    (`SplineComponent.SetSplinePointType` (`self.Shape`) _index (`self.SplineType`) true)))

(fn `UserConstructionScript`
  (locals (Distance :type "Float (double-precision)"))
  (bind _scale_x (`KismetMathLibrary.BreakVector` (`self.Scale`)))
  (bind _mesh (`self.Mesh`))
  (bind (_scale_x_2 _scale_y _scale_z) (`KismetMathLibrary.BreakVector` (`self.Scale`)))
  (bind _shape (`self.Shape`))
  (bind (_returnvalue_origin _returnvalue_boxextent) (`KismetMathLibrary.BreakBoxSphereBounds` (`StaticMesh.GetBounds` (`self.SplineMesh`))))
  (bind _returnvalue_x (`KismetMathLibrary.BreakVector` (* (* _returnvalue_boxextent 2) _scale_x)))
  (`PrimitiveComponent.SetRenderCustomDepth` _mesh (`self.Stencil`))
  (`PrimitiveComponent.SetCustomDepthStencilValue` _mesh (`self.Semantic Index`))
  (`StaticMeshComponent.SetStaticMesh` (`self.Mesh`) (`self.SplineMesh`))
  (set `self.TotalInstances` 0)
  (`SplineComponent.SetClosedLoop` (`self.Shape`) (`self.Closed`) true)
  (if (`self.Live Update`)
    (if (not (`self.StraightenMeshes`))
      (for _index (range (`SplineComponent.GetNumberOfSplinePoints` (`self.Shape`)))
        (`self.GenerateSplinePart` (`self.SurfaceOffset`) (`self.SplineMesh`) _index))
      (else
        (for _index_2 (range (`SplineComponent.GetNumberOfSplinePoints` (`self.Shape`)))
          (bind _returnvalue (`SplineComponent.GetDistanceAlongSplineAtSplinePoint` _shape _index_2))
          (bind (_scale _parts) (`self.CalculateScale` (- (`SplineComponent.GetDistanceAlongSplineAtSplinePoint` _shape (+ _index_2 1)) _returnvalue) _returnvalue_x))
          (for _index_3 (range _parts)
            (bind (_returnvalue_location _returnvalue_rotation) (`KismetMathLibrary.BreakTransform` (`SplineComponent.GetTransformAtDistanceAlongSpline` (`self.Shape`) (+ (* _index_3 (* _scale _returnvalue_x)) _returnvalue) "Local" true)))
            (`InstancedStaticMeshComponent.AddInstance` (`self.Mesh`) (`KismetMathLibrary.MakeTransform` _returnvalue_location _returnvalue_rotation (`KismetMathLibrary.MakeVector` (+ (- _scale 1.0) _scale_x_2) _scale_y _scale_z)))))))))