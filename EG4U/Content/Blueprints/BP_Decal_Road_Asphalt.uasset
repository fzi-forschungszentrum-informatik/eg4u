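; Asphalt spline decal road actor that stores an ID and connection IDs for linking to other roads of its class.
; MakeConnections gathers roads with matching IDs and checks for existing back-links.
; GetClosestEndpoints finds the nearest pair of spline ends between two roads.
; The code that would spawn ground-hugging connector roads between those ends, excluded from the main render pass, is disconnected and never runs.
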(fn `Get Closest Endpoints`
  (params (`Other Spline` :type "SplineComponent Object Reference"))
  (returns (`My Endpoint` :type Integer) (`Other Endpoint` :type Integer))
  (locals (my :type Integer :default 0) (other :type Integer :default 0))
  (bind _spline (`self.Spline`))
  (bind _other_spline (`local.Other Spline`))
  (bind _returnvalue (`SplineComponent.GetLocationAtSplinePoint` _other_spline 0 "World"))
  (bind _returnvalue_2 (`SplineComponent.GetLocationAtSplinePoint` _spline 0 "World"))
  (bind _returnvalue_3 (`KismetMathLibrary.Vector_Distance` _returnvalue_2 _returnvalue))
  (bind _returnvalue_4 (- (`SplineComponent.GetNumberOfSplinePoints` (`local.Other Spline`)) 1))
  (bind _returnvalue_5 (- (`SplineComponent.GetNumberOfSplinePoints` (`self.Spline`)) 1))
  (bind _returnvalue_6 (`SplineComponent.GetLocationAtSplinePoint` _other_spline (- (`SplineComponent.GetNumberOfSplinePoints` (`local.Other Spline`)) 1) "World"))
  (bind _returnvalue_7 (`SplineComponent.GetLocationAtSplinePoint` _spline (- (`SplineComponent.GetNumberOfSplinePoints` (`self.Spline`)) 1) "World"))
  (bind _returnvalue_8 (`KismetMathLibrary.Vector_Distance` _returnvalue_7 _returnvalue_6))
  (bind _returnvalue_9 (`KismetMathLibrary.Vector_Distance` _returnvalue_7 _returnvalue))
  (bind _returnvalue_10 (`KismetMathLibrary.Vector_Distance` _returnvalue_2 _returnvalue_6))
  (bind _returnvalue_11 (< _returnvalue_9 _returnvalue_8))
  (bind _returnvalue_12 (< _returnvalue_3 _returnvalue_10))
  (if (< (`KismetMathLibrary.SelectFloat` _returnvalue_3 _returnvalue_10 _returnvalue_12) (`KismetMathLibrary.SelectFloat` _returnvalue_9 _returnvalue_8 _returnvalue_11))
    (if _returnvalue_12
      (set `local.my` 0)
      (set `local.other` 0)
      (else
        (set `local.my` 0)
        (set `local.other` _returnvalue_4)))
    (elif _returnvalue_11
      (set `local.my` _returnvalue_5)
      (set `local.other` 0)
      (else
        (set `local.my` _returnvalue_5)
        (set `local.other` _returnvalue_4))))
  (return (`local.my`) (`local.other`)))

(fn `Make Connections`
  (params (VTs :type "Array of RuntimeVirtualTexture Object Reference"))
  (returns (`Output roads` :type "Array of /Game/DecalRoadsRVT/BP_DecalRoad_Asphalt Object Reference"))
  (locals (`New Roads` :type "Array of /Game/DecalRoadsRVT/BP_DecalRoad_Asphalt Object Reference") (`Temp Points` :type "Array of Vector Structure"))
  (bind _outactors (`GameplayStatics.GetAllActorsOfClass` "/Game/DecalRoadsRVT/BP_DecalRoad_Asphalt.BP_DecalRoad_Asphalt_C"))
  (`|ExecutionSequence`
    (:`then_0`
      (for _array_element _outactors
        (for _array_element_2 (`self.Connections`)
          (if (== _array_element_2 (`/Game/DecalRoadsRVT/BP_DecalRoad_Asphalt.ID` _array_element))
            (`KismetArrayLibrary.Array_Add` (`self.Connecting Roads`) _array_element)))))
    (:`then_1`
      (for (_array_element_3 _array_index) (`self.Connecting Roads`)
        (set `self.Self Connected?` false)
        (for _array_element_4 (`/Game/DecalRoadsRVT/BP_DecalRoad_Asphalt.Connected Roads` _array_element_3)
          (set `self.Self Connected?` (== (`/Game/DecalRoadsRVT/BP_DecalRoad_Asphalt.ID` _array_element_4) (`self.ID`))))))))

(fn `Set Connections`
  (params (In :type "Array of Integer"))
  (for _array_element In
    (`KismetArrayLibrary.Array_Add` (`self.Connections`) _array_element)))

(fn `Set ID`
  (params (ID :type Integer))
  (set `self.ID` ID))

(fn `UserConstructionScript`
  (`parent.UserConstructionScript`))