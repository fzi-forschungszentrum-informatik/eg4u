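; Procedural building facade actor that stacks BP_FloorPattern actors along a footprint and caps them with a roof.
; Construction derives ground, middle and roof level heights from the tallest mesh in each set, and generates the facade upon first finding an OpenStreetMap_MeshBuilder.
; Each generation clears previous floors, optionally randomizes seeds, then spawns and attaches floors.
; The mesh builder supplies roof geometry for a procedural mesh component.
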(fn `Generate Facade`
  (params (Footprint :type "Array of Vector Structure") (Reversed :type Boolean))
  (locals (CurrentFloor :type "/EG4U/Blueprints/BP_FloorPattern Object Reference") (`current Index` :type Integer))
  (bind _current_index (`local.current Index`))
  (bind (_returnvalue_x _returnvalue_y _returnvalue_z) (`KismetMathLibrary.BreakVector` (`self.K2_GetActorLocation` self)))
  (bind _returnvalue (+ _returnvalue_z (`self.height`)))
  (set `self.Footprint` Footprint)
  (set `self.Reversed` Reversed)
  (if (`self.Random Pattern`)
    (`self.Randomize`))
  (`self.Reset`)
  (for _index (range (+ (`self.Floors`) 1))
    (set `local.current Index` _index)
    (`|ExecutionSequence`
      (:`then_0`
        (bind _returnvalue_2 (`|SpawnActorFromClass` "/EG4U/Blueprints/BP_FloorPattern.BP_FloorPattern_C" (`KismetMathLibrary.MakeTransform` (`KismetMathLibrary.MakeVector` _returnvalue_x _returnvalue_y _returnvalue) (`self.K2_GetActorRotation` self)) "Undefined" "OverrideRootScale" null null))
        (set `local.CurrentFloor` _returnvalue_2)
        (`KismetArrayLibrary.Array_Add` (`self.FloorActors`) (`local.CurrentFloor`))
        (`/EG4U/Blueprints/BP_FloorPattern.SetFootprint` (`local.CurrentFloor`) (`self.Footprint`) _returnvalue (`self.Reversed`)))
      (:`then_1`
        (if (== _current_index 0)
          (set `self.height` (+ (`self.height`) (`self.height ground`)))
          (set `/EG4U/Blueprints/BP_FloorPattern.Meshes` (`self.Ground Level`) (`local.CurrentFloor`)) ; Ground Level
          (set `/EG4U/Blueprints/BP_FloorPattern.GenerateWindow` (`self.Generate Window Ground Floor`) (`local.CurrentFloor`))
          (set `/EG4U/Blueprints/BP_FloorPattern.Random Seed` (`self.Ground Seed`) (`local.CurrentFloor`))
          (elif (== _current_index (`self.Floors`))
            (set `self.height` (+ (`self.height`) (`self.height roof`)))
            (set `/EG4U/Blueprints/BP_FloorPattern.Meshes` (`self.Roof Level`) (`local.CurrentFloor`)) ; Roof Level
            (set `/EG4U/Blueprints/BP_FloorPattern.GenerateWindow` (`self.Generate Window Roof Floor`) (`local.CurrentFloor`))
            (set `/EG4U/Blueprints/BP_FloorPattern.Random Seed` (`self.Roof Seed`) (`local.CurrentFloor`))
            (else
              (set `self.height` (+ (`self.height`) (`self.height middle`)))
              (set `/EG4U/Blueprints/BP_FloorPattern.Meshes` (`self.Middle Levels`) (`local.CurrentFloor`)) ; Middle Level
              (set `/EG4U/Blueprints/BP_FloorPattern.GenerateWindow` (`self.Generate Window Middle Floors`) (`local.CurrentFloor`))
              (set `/EG4U/Blueprints/BP_FloorPattern.Random Seed` (`self.Middle Seed`) (`local.CurrentFloor`)))))
        (`/EG4U/Blueprints/BP_FloorPattern.Generate Floor` (`local.CurrentFloor`)))
      (:`then_2`
        (`self.K2_AttachToActor` (`local.CurrentFloor`) self "None" "KeepWorld" "KeepWorld" "KeepWorld" false))))
  (`self.GenerateRoof`))

(fn `GenerateRoof`
  (if (`KismetSystemLibrary.IsValid` (`self.ParentGenerator`))
    (`self.RemoveRoof`)
    (bind _returnvalue (`AddComponent|NODE_AddProceduralMeshComponent-0`))
    (set `self.RoofMesh` _returnvalue)
    (bind _returnvalue_2 (`OpenStreetMap_Generator.GenerateRoof` (`self.ParentGenerator`) (`self.Footprint`) (`self.Osm Tags`) (`self.Roof Type`) (- (`self.height`) 50.0) (`self.Roof Size`)))
    (`ProceduralMeshComponent.CreateMeshSection_LinearColor` :`self` (`self.RoofMesh`) :`Vertices` (break `OpenStreetMap_Generator_MeshInfo` _returnvalue_2) :`Triangles` (`.triangles` (break `OpenStreetMap_Generator_MeshInfo` _returnvalue_2)) :`UV0` (`.uv_coords` (break `OpenStreetMap_Generator_MeshInfo` _returnvalue_2)))
    (`PrimitiveComponent.SetMaterial` (`self.RoofMesh`) 0 (`self.RoofMaterial`))))

(fn `Randomize`
  (bind _main_seed (`self.Main Seed`))
  (bind _main_seed_2 (`self.Main Seed`))
  (bind _main_seed_3 (`self.Main Seed`))
  (`|ExecutionSequence`
    (:`then_0`
      (set `self.Ground Seed` (`KismetMathLibrary.RandomIntegerFromStream` 2147483647 (`self.Stream`)))
      (`KismetMathLibrary.SetRandomStreamSeed` (`self.Stream`) _main_seed)
      (set `self.Main Seed` (+ _main_seed 1)))
    (:`then_1`
      (set `self.Middle Seed` (`KismetMathLibrary.RandomIntegerFromStream` 2147483647 (`self.Stream`)))
      (`KismetMathLibrary.SetRandomStreamSeed` (`self.Stream`) _main_seed_3)
      (set `self.Main Seed` (+ _main_seed_3 1)))
    (:`then_2`
      (set `self.Roof Seed` (`KismetMathLibrary.RandomIntegerFromStream` 2147483647 (`self.Stream`)))
      (`KismetMathLibrary.SetRandomStreamSeed` (`self.Stream`) _main_seed_2)
      (set `self.Main Seed` (+ _main_seed_2 1))
      (set `self.RoofMaterial` (`|GetArrayItem` (`self.RoofMaterials`) (`KismetMathLibrary.RandomIntegerInRange` 0 (`KismetArrayLibrary.Array_LastIndex` (`self.RoofMaterials`))))))))

(fn `Regenerate`
  (locals (CurrentFloor :type "/EG4U/Blueprints/BP_FloorPattern Object Reference") (`current Index` :type Integer))
  (bind _current_index (`local.current Index`))
  (bind (_returnvalue_x _returnvalue_y _returnvalue_z) (`KismetMathLibrary.BreakVector` (`self.K2_GetActorLocation` self)))
  (bind _returnvalue (+ _returnvalue_z (`self.height`)))
  (if (`self.Random Pattern`)
    (`self.Randomize`))
  (`self.Reset`)
  (for _index (range (+ (`self.Floors`) 1))
    (set `local.current Index` _index)
    (`|ExecutionSequence`
      (:`then_0`
        (bind _returnvalue_2 (`|SpawnActorFromClass` "/EG4U/Blueprints/BP_FloorPattern.BP_FloorPattern_C" (`KismetMathLibrary.MakeTransform` (`KismetMathLibrary.MakeVector` _returnvalue_x _returnvalue_y _returnvalue) (`self.K2_GetActorRotation` self)) "Undefined" "OverrideRootScale" null null))
        (set `local.CurrentFloor` _returnvalue_2)
        (`KismetArrayLibrary.Array_Add` (`self.FloorActors`) (`local.CurrentFloor`))
        (`/EG4U/Blueprints/BP_FloorPattern.SetFootprint` (`local.CurrentFloor`) (`self.Footprint`) _returnvalue (`self.Reversed`)))
      (:`then_1`
        (if (== _current_index 0)
          (set `self.height` (+ (`self.height`) (`self.height ground`)))
          (set `/EG4U/Blueprints/BP_FloorPattern.Meshes` (`self.Ground Level`) (`local.CurrentFloor`)) ; Ground Level
          (set `/EG4U/Blueprints/BP_FloorPattern.GenerateWindow` (`self.Generate Window Ground Floor`) (`local.CurrentFloor`))
          (set `/EG4U/Blueprints/BP_FloorPattern.Random Seed` (`self.Ground Seed`) (`local.CurrentFloor`))
          (elif (== _current_index (`self.Floors`))
            (set `self.height` (+ (`self.height`) (`self.height roof`)))
            (set `/EG4U/Blueprints/BP_FloorPattern.Meshes` (`self.Roof Level`) (`local.CurrentFloor`)) ; Roof Level
            (set `/EG4U/Blueprints/BP_FloorPattern.GenerateWindow` (`self.Generate Window Roof Floor`) (`local.CurrentFloor`))
            (set `/EG4U/Blueprints/BP_FloorPattern.Random Seed` (`self.Roof Seed`) (`local.CurrentFloor`))
            (else
              (set `self.height` (+ (`self.height`) (`self.height middle`)))
              (set `/EG4U/Blueprints/BP_FloorPattern.Meshes` (`self.Middle Levels`) (`local.CurrentFloor`)) ; Middle Level
              (set `/EG4U/Blueprints/BP_FloorPattern.GenerateWindow` (`self.Generate Window Middle Floors`) (`local.CurrentFloor`))
              (set `/EG4U/Blueprints/BP_FloorPattern.Random Seed` (`self.Middle Seed`) (`local.CurrentFloor`)))))
        (`/EG4U/Blueprints/BP_FloorPattern.Generate Floor` (`local.CurrentFloor`)))
      (:`then_2`
        (`self.K2_AttachToActor` (`local.CurrentFloor`) self "None" "KeepWorld" "KeepWorld" "KeepWorld" false))))
  (`self.GenerateRoof`))

(fn `RemoveRoof`
  (bind _roofmesh (`self.RoofMesh`))
  (`ProceduralMeshComponent.ClearAllMeshSections` _roofmesh)
  (`ActorComponent.K2_DestroyComponent` _roofmesh))

(fn `Reset`
  (bind _flooractors (`self.FloorActors`))
  (`self.RemoveRoof`)
  (for _array_element _flooractors
    (`/EG4U/Blueprints/BP_FloorPattern.Clear` _array_element)
    (`self.K2_DestroyActor` _array_element))
  (`KismetArrayLibrary.Array_Clear` _flooractors)
  (set `self.height` 0.0)
  (bind (_arrayindex _arrayelement) (`/Engine/EditorBlueprintResources/StandardMacros.ReverseForEachLoop` (`self.GetAttachedActors` true))
    (:`LoopBody`
      (`self.K2_DestroyActor` _arrayelement))
    (:`Completed`
      (`ActorComponent.K2_DestroyComponent` (`self.RoofMesh`)))))

(fn `UserConstructionScript`
  (locals (ground :type "Array of Float (double-precision)") (roof :type "Array of Float (double-precision)") (middle :type "Array of Float (double-precision)"))
  (for _array_element (`self.Ground Level`)
    (`KismetArrayLibrary.Array_Add` (`local.ground`) (.z (`.BoxExtent` (`KismetMathLibrary.BreakBoxSphereBounds` (`StaticMesh.GetBounds` _array_element))))))
  (for _array_element_2 (`self.Roof Level`)
    (`KismetArrayLibrary.Array_Add` (`local.roof`) (.z (`.BoxExtent` (`KismetMathLibrary.BreakBoxSphereBounds` (`StaticMesh.GetBounds` _array_element_2))))))
  (for _array_element_3 (`self.Middle Levels`)
    (`KismetArrayLibrary.Array_Add` (`local.middle`) (.z (`.BoxExtent` (`KismetMathLibrary.BreakBoxSphereBounds` (`StaticMesh.GetBounds` _array_element_3))))))
  (set `self.height ground` (* 2 (`.MaxValue` (`KismetMathLibrary.MaxOfFloatArray` (`local.ground`)))))
  (set `self.height middle` (* 2 (`.MaxValue` (`KismetMathLibrary.MaxOfFloatArray` (`local.middle`)))))
  (set `self.height roof` (* 2 (`.MaxValue` (`KismetMathLibrary.MaxOfFloatArray` (`local.roof`)))))
  (if (not (`KismetSystemLibrary.IsValid` (`self.ParentGenerator`)))
    (bind _returnvalue (`GameplayStatics.GetActorOfClass` "/EG4U/OpenStreetMap_MeshBuilder.OpenStreetMap_MeshBuilder_C"))
    (if (`KismetSystemLibrary.IsValid` _returnvalue)
      (set `self.ParentGenerator` _returnvalue)
      (`self.Generate Facade` (`self.Footprint`) (`self.Reversed`)))))