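; BP_FloorPattern procedurally builds one floor of modular meshes along a linear spline footprint, which SetFootprint can supply from points and a height.
; The construction script rebuilds it, filling each segment with instanced static meshes.
; With RandomPattern, a seeded stream picks modules for half the segment and appends them reversed, aiming for symmetry.
; Modules are stretched along X to fit exactly, with optional window instances offset and scaled to each.
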(fn `Calculate number of meshes`
  (params (MeshLength :type "Float (double-precision)") (TotalDistance :type "Float (double-precision)"))
  (returns (Scale :type "Float (double-precision)") (`Number of Meshes` :type Integer))
  (bind _returnvalue (`KismetMathLibrary.FTrunc` (/ TotalDistance MeshLength)))
  (bind _returnvalue_2 (* _returnvalue MeshLength))
  (if (or (== _returnvalue_2 0.0) (== TotalDistance 0.0))
    (return (/ TotalDistance MeshLength) 0)
    (else
      (return (/ TotalDistance _returnvalue_2) (- _returnvalue 1)))))

(fn `CalculateScale`
  (params (SplineLength :type "Float (double-precision)") (MeshSize :type "Float (double-precision)"))
  (returns (Scale :type "Float (double-precision)") (Parts :type Integer))
  (bind (_remainder _returnvalue) (`KismetMathLibrary.FMod` SplineLength MeshSize))
  (bind _returnvalue_2 (!= _returnvalue 0))
  (return (select `bool` _returnvalue_2 :`false` (/ _remainder MeshSize) :`true` (/ SplineLength MeshSize)) (select `bool` _returnvalue_2 :`true` _returnvalue)))

(fn `Clear`
  (bind _windowmesh (`self.WindowMesh`))
  (for _array_element (`self.ISM`)
    (`InstancedStaticMeshComponent.ClearInstances` _array_element)
    (`ActorComponent.K2_DestroyComponent` _array_element))
  (`KismetArrayLibrary.Array_Clear` (`self.ISM`))
  (`InstancedStaticMeshComponent.ClearInstances` _windowmesh)
  (`ActorComponent.K2_DestroyComponent` _windowmesh))

(fn `ConfigureAssets`
  (`KismetArrayLibrary.Array_Clear` (`QuickStripPacking.items_in` (`self.QuickStripPacking`)))
  (for (_array_element _array_index) (`self.Meshes`)
    (`KismetArrayLibrary.Array_Add` (`QuickStripPacking.items_in` (`self.QuickStripPacking`)) (make `QuickStripPacking_Item` _array_index (* 2 (.x (`.BoxExtent` (`KismetMathLibrary.BreakBoxSphereBounds` (`StaticMesh.GetBounds` _array_element)))))))))

(fn `Generate Floor`
  (bind _meshbounds (`self.MeshBounds`))
  (bind _shape (`self.Shape`))
  (bind (_returnvalue_origin _returnvalue_boxextent) (`KismetMathLibrary.BreakBoxSphereBounds` (`StaticMesh.GetBounds` (`self.Window`))))
  (`KismetMathLibrary.SetRandomStreamSeed` (`self.Stream`) (`self.Random Seed`))
  (`self.Clear`)
  (if (`self.GenerateWindow`)
    (bind _returnvalue (`AddComponent|NODE_AddInstancedStaticMeshComponent-4`))
    (bind _output_get (set `self.WindowMesh` _returnvalue))
    (`StaticMeshComponent.SetStaticMesh` _output_get (`self.Window`)))
  (set `self.CurrentLength` 0.0)
  (`KismetArrayLibrary.Array_Clear` (`self.MeshBounds`))
  (`KismetArrayLibrary.Array_Clear` (`self.ISM`))
  (for _index (range (+ (- (`SplineComponent.GetNumberOfSplinePoints` (`self.Shape`)) 2) 1))
    (set `self.CurrentLength` 0.0)
    (`KismetArrayLibrary.Array_Clear` (`self.Pattern`))
    (bind _location (`SplineComponent.GetLocationAndTangentAtSplinePoint` _shape (+ _index 1) "Local"))
    (bind _location_2 (`SplineComponent.GetLocationAndTangentAtSplinePoint` _shape _index "Local"))
    (bind _returnvalue_2 (`KismetMathLibrary.VSize` (- _location _location_2)))
    (`self.GeneratePattern` _returnvalue_2)
    (bind _totallength (`self.PrepareAssets`))
    (set `self.AssetWidth` _totallength)
    (set `self.SplineLength` _returnvalue_2)
    (bind _output_get_2 (set `self.Remainder` (/ _returnvalue_2 (`self.AssetWidth`))))
    (for _array_element (`self.Pattern`)
      (bind _returnvalue_3 (`KismetMathLibrary.FindLookAtRotation` _location_2 _location))
      (bind _returnvalue_4 (`KismetMathLibrary.TransformLocation` (`KismetMathLibrary.MakeTransform` _location_2 _returnvalue_3) (`KismetMathLibrary.MakeVector` (`self.CurrentLength`))))
      (`InstancedStaticMeshComponent.AddInstance` (`|GetArrayItem` (`self.ISM`) _array_element) (`KismetMathLibrary.MakeTransform` _returnvalue_4 _returnvalue_3 (`KismetMathLibrary.MakeVector` _output_get_2 1.0 1.0)))
      (if (`self.GenerateWindow`)
        (bind (_output_x _output_y) (`KismetMathLibrary.BreakVector` (`|GetArrayItem` _meshbounds _array_element)))
        (bind (_returnvalue_x _returnvalue_y _returnvalue_z) (`KismetMathLibrary.BreakVector` (/ (`|GetArrayItem` _meshbounds _array_element) _returnvalue_boxextent)))
        (`InstancedStaticMeshComponent.AddInstance` (`self.WindowMesh`) (`KismetMathLibrary.MakeTransform` (`KismetMathLibrary.TransformLocation` (`KismetMathLibrary.MakeTransform` _returnvalue_4 _returnvalue_3) (`KismetMathLibrary.MakeVector` 0.0 (* _output_y -2.0))) _returnvalue_3 (`KismetMathLibrary.MakeVector` (* (`self.Remainder`) _returnvalue_x) 0.01 _returnvalue_z))))
      (set `self.CurrentLength` (+ (* (* 2 _output_x) _output_get_2) (`self.CurrentLength`))))))

(fn `GeneratePattern`
  (params (SplineLength :type "Float (double-precision)"))
  (locals (sum :type "Float (double-precision)" :default 0.0) (current_length :type "Float (double-precision)" :default 0.0) (indexreverse :type "Array of Integer"))
  (bind _returnvalue (/ SplineLength 2.0))
  (bind _indexreverse (`local.indexreverse`))
  (bind _returnvalue_2 (`KismetMathLibrary.RandomIntegerInRangeFromStream` 0 (`KismetArrayLibrary.Array_LastIndex` (`self.MeshBounds`)) (`self.Stream`)))
  (bind _output_x (`KismetMathLibrary.BreakVector` (`|GetArrayItem` (`self.MeshBounds`) _returnvalue_2)))
  (bind _output_x_2 (`KismetMathLibrary.BreakVector` (`|GetArrayItem` (`self.MeshBounds`) (`KismetMathLibrary.Clamp` (`KismetArrayLibrary.Array_LastIndex` (`local.indexreverse`)) 0 300))))
  (for _array_element (`self.Meshes`)
    (bind _returnvalue_3 (`AddComponent|NODE_AddInstancedStaticMeshComponent-3`))
    (`StaticMeshComponent.SetStaticMesh` _returnvalue_3 _array_element)
    (`KismetArrayLibrary.Array_Add` (`self.ISM`) _returnvalue_3)
    (bind (_returnvalue_origin _returnvalue_boxextent) (`KismetMathLibrary.BreakBoxSphereBounds` (`StaticMesh.GetBounds` _array_element)))
    (`KismetArrayLibrary.Array_Add` (`self.MeshBounds`) _returnvalue_boxextent)
    (set `local.sum` (.x _returnvalue_boxextent)))
  (if (`self.RandomPattern`)
    (`KismetArrayLibrary.Array_Add` (`self.Pattern`))
    (bind _output_get (set `local.current_length` (+ (`local.current_length`) (* 2 _output_x_2))))
    (while (< _output_get _returnvalue)
      (`KismetArrayLibrary.Array_Add` (`local.indexreverse`) _returnvalue_2)
      (set `local.current_length` (+ (`local.current_length`) (* 2 _output_x))))
    (`KismetArrayLibrary.Array_Append` (`self.Pattern`) (`local.indexreverse`))
    (if (not (> (- _returnvalue _output_get) _output_x_2))
      (`KismetArrayLibrary.Array_RemoveItem` _indexreverse (`KismetArrayLibrary.Array_LastIndex` _indexreverse)))
    (`KismetArrayLibrary.Array_Reverse` (`local.indexreverse`))
    (`KismetArrayLibrary.Array_Append` (`self.Pattern`) (`local.indexreverse`))))

(fn `PrepareAssets`
  (returns (TotalLength :type "Float (double-precision)"))
  (locals (t :type "Float (double-precision)"))
  (for _index (range (`SplineComponent.GetNumberOfSplinePoints` (`self.Shape`)))
    (`SplineComponent.SetSplinePointType` (`self.Shape`) _index "Linear" true)
    (for _array_element (`self.Pattern`)
      (bind _output_x (`KismetMathLibrary.BreakVector` (`|GetArrayItem` (`self.MeshBounds`) _array_element)))
      (set `local.t` (+ (* 2 _output_x) (`local.t`))))
    (return (`local.t`))))

(fn `SetFootprint`
  (params (Points :type "Array of Vector Structure") (Height :type "Float (double-precision)") (Reverse :type Boolean))
  (locals (Footprint :type "Array of Vector Structure"))
  (bind _footprint (`local.Footprint`))
  (bind _shape (`self.Shape`))
  (if Reverse
    (for _array_element Points
      (`KismetArrayLibrary.Array_Add` _footprint (`KismetMathLibrary.MakeVector` (.x _array_element) (.y _array_element) Height)))
    (`SplineComponent.SetSplinePoints` _shape (`local.Footprint`) "World" false :!label _label)
    (for _index (range (`SplineComponent.GetNumberOfSplinePoints` _shape))
      (`SplineComponent.SetSplinePointType` (`self.Shape`) _index "Linear" true))
    (else
      (bind (_arrayindex _arrayelement) (`/Engine/EditorBlueprintResources/StandardMacros.ReverseForEachLoop` Points)
        (:`LoopBody`
          (`KismetArrayLibrary.Array_Add` _footprint (`KismetMathLibrary.MakeVector` (.x _arrayelement) (.y _arrayelement) Height)))
        (:`Completed`
          (goto _label))))))

(fn `UserConstructionScript`
  (`self.Generate Floor`))