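; BP_Repeater is a construction-time tool that repeats a static mesh at regular intervals along a spline.
; Its construction script adds an instanced static mesh component, then steps along the spline by Space until reaching its length.
; Each instance takes the local spline location and rotation, offset by adding RelativeTransformRotation per axis, and ignores spline scale.
; The event graph holds only disabled stub events, so there is no runtime logic.
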(fn `UserConstructionScript`
  (bind _current_length (`self.Current Length`))
  (bind (_relative_transform_rotation_roll _relative_transform_rotation_pitch _relative_transform_rotation_yaw) (`KismetMathLibrary.BreakRotator` (`self.Relative Transform Rotation`)))
  (bind _returnvalue (`SplineComponent.GetTransformAtDistanceAlongSpline` (`self.Spline`) _current_length "Local" false))
  (bind _returnvalue_2 (`AddComponent|NODE_AddInstancedStaticMeshComponent-0`))
  (`StaticMeshComponent.SetStaticMesh` _returnvalue_2 (`self.Mesh`))
  (while (< _current_length (`SplineComponent.GetSplineLength` (`self.Spline`)))
    (`InstancedStaticMeshComponent.AddInstance` _returnvalue_2 (`KismetMathLibrary.MakeTransform` (.location _returnvalue) (`KismetMathLibrary.MakeRotator` (+ _relative_transform_rotation_roll (.roll (.rotation _returnvalue))) (+ _relative_transform_rotation_pitch (.pitch (.rotation _returnvalue))) (+ _relative_transform_rotation_yaw (.yaw (.rotation _returnvalue)))) (.scale _returnvalue)))
    (set `self.Current Length` (+ (`self.Current Length`) (`self.Space`)))))