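; Building facade generator (OSM by name) with a GenerateFloor function that lines a spline footprint with instanced meshes, stretched to fit each straight segment.
; MakeRoof triggers a roof polygon from the spline points, raised by the mesh height.
; A temporary StreetMap component triangulates it into a procedural mesh, with a reversed-index second section for double-sided faces, optionally saved as an asset.
; Construction script and event graph are empty.
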(fn `Calculate number of meshes`
  (params (MeshLength :type "Float (double-precision)") (TotalDistance :type "Float (double-precision)"))
  (returns (Scale :type "Float (double-precision)") (`Number of Meshes` :type Integer))
  (bind _returnvalue (/ TotalDistance MeshLength))
  (bind _returnvalue_2 (`KismetMathLibrary.FTrunc` _returnvalue))
  (bind _returnvalue_3 (* _returnvalue_2 MeshLength))
  (if (or (== _returnvalue_3 0.0) (== TotalDistance 0.0))
    (return _returnvalue 0)
    (else
      (return (/ TotalDistance _returnvalue_3) (- _returnvalue_2 1)))))

(fn `CalculateScale`
  (params (SplineLength :type "Float (double-precision)") (MeshSize :type "Float (double-precision)"))
  (returns (Scale :type "Float (double-precision)") (Parts :type Integer))
  (bind (_remainder _returnvalue) (`KismetMathLibrary.FMod` SplineLength MeshSize))
  (bind _returnvalue_2 (!= _returnvalue 0))
  (return (select `bool` _returnvalue_2 :`false` (/ _remainder MeshSize) :`true` (/ SplineLength MeshSize)) (select `bool` _returnvalue_2 :`true` _returnvalue)))

(fn `Clear`
  (bind _proceduraltriangles (`self.ProceduralTriangles`))
  (`KismetArrayLibrary.Array_Clear` (`self.X3`))
  (`KismetArrayLibrary.Array_Clear` (`self.Vertices`))
  (for _array_element _proceduraltriangles
    (`ActorComponent.K2_DestroyComponent` _array_element))
  (`KismetArrayLibrary.Array_Clear` _proceduraltriangles)
  (`ActorComponent.K2_DestroyComponent` (`self.ProceduralMesh`)))

(fn `Generate Floor`
  (params (ISM :type "InstancedStaticMeshComponent Object Reference") (Mesh :type "StaticMesh Object Reference"))
  (bind (_returnvalue_origin _returnvalue_boxextent) (`KismetMathLibrary.BreakBoxSphereBounds` (`StaticMesh.GetBounds` Mesh)))
  (bind _shape (`self.Shape`))
  (bind _shape_2 (`self.Shape`))
  (bind (_mesh_bounds_x _mesh_bounds_y _mesh_bounds_z) (`KismetMathLibrary.BreakVector` (`self.Mesh Bounds`)))
  (bind _mesh_bounds_x_2 (`KismetMathLibrary.BreakVector` (`self.Mesh Bounds`)))
  (`self.Clear`)
  (set `self.Mesh Bounds` _returnvalue_boxextent)
  (for _index (range (+ (- (`SplineComponent.GetNumberOfSplinePoints` _shape) 2) 1))
    (`SplineComponent.SetSplinePointType` _shape _index "Linear" true)
    ;[1 0 0] Straight Middle Segments
    (set `self.SurfaceOffset` (* 2 _mesh_bounds_z))
    (bind _location (`SplineComponent.GetLocationAndTangentAtSplinePoint` _shape_2 (+ _index 1) "Local"))
    (bind _location_2 (`SplineComponent.GetLocationAndTangentAtSplinePoint` _shape_2 _index "Local"))
    (bind (_scale _number_of_meshes) (`self.Calculate number of meshes` (* 2 _mesh_bounds_x) (`KismetMathLibrary.VSize` (- _location _location_2))))
    (for _index_2 (range (+ _number_of_meshes 1))
      (bind _returnvalue (`KismetMathLibrary.FindLookAtRotation` _location_2 _location))
      (set `self.FinalTransform` _returnvalue)
      (`InstancedStaticMeshComponent.AddInstance` ISM (`KismetMathLibrary.MakeTransform` (`KismetMathLibrary.TransformLocation` (`KismetMathLibrary.MakeTransform` (+ (* (* (`KismetMathLibrary.Conv_RotatorToVector` _returnvalue) _index_2) (* _scale (* 2 _mesh_bounds_x_2))) _location_2) _returnvalue) (0.0 0.0 0.0)) (`self.FinalTransform`) (`KismetMathLibrary.MakeVector` _scale 1.0 1.0)))))
  (if (`self.MakeRoof`)
    (`self.Generate Polygon`)))

(fn `Generate Polygon`
  (locals (Points2D :type "Array of Vector2D Structure") (SmartDistribution :type Boolean))
  (bind _shape (`self.Shape`))
  (bind _returnvalue (`SplineComponent.GetNumberOfSplinePoints` _shape))
  ;[1 0 1] Polygon Generation
  (for _index (range _returnvalue)
    (bind (_returnvalue_x _returnvalue_y _returnvalue_z) (`KismetMathLibrary.BreakVector` (`SplineComponent.GetLocationAtSplinePoint` _shape _index "Local")))
    (`KismetArrayLibrary.Array_Add` (`local.Points2D`) (`KismetMathLibrary.MakeVector2D` _returnvalue_x _returnvalue_y))
    (`KismetArrayLibrary.Array_Add` (`self.X3`) _returnvalue_z))
  (if (>= _returnvalue 3)
    (bind _polygon (`self.Make Polygon` (`local.Points2D`) (`self.X3`) (`self.SurfaceOffset`)))
    (if (`self.SaveProceduralSurface`)
      (`StreetMapComponent.SaveProceduralMesh` _polygon (`self.OutputDirectory`) (`self.OutputName`)))))

(fn `Make Polygon`
  (params (InPoints :type "Array of Vector2D Structure") (Z :type "Array of Float (double-precision)") (Height :type "Float (double-precision)"))
  (returns (Polygon :type "ProceduralMeshComponent Object Reference"))
  (locals (Points2D_Reversed :type "Array of Integer") (Vertices_Reversed :type "Array of Vector Structure"))
  (bind _vertices (`self.Vertices`))
  (bind _returnvalue (`AddComponent|NODE_AddStreetMapComponent-1`))
  (bind (_tempindices _triangulatedindices) (`StreetMapComponent.TriangulatePolygonInPlace` _returnvalue InPoints))
  (bind _returnvalue_2 (`AddComponent|NODE_AddProceduralMeshComponent-2`))
  (`KismetArrayLibrary.Array_Add` (`self.ProceduralTriangles`) _returnvalue_2)
  (for (_array_element _array_index) InPoints
    (`KismetArrayLibrary.Array_Set` (`self.Vertices`) _array_index (`KismetMathLibrary.MakeVector` (`KismetMathLibrary.BreakVector2D` _array_element) (`.Y` (`KismetMathLibrary.BreakVector2D` _array_element)) (+ (`|GetArrayItem` Z _array_index) Height)) true))
  (`/Game/ProceduralBuildingGenerator/Blueprints/PBG_Data/PolygonX_Core.TriangulatePolygon` (`self.Vertices`))
  (`ProceduralMeshComponent.CreateMeshSection_LinearColor` :`self` _returnvalue_2 :`Vertices` (`self.Vertices`) :`Triangles` _triangulatedindices)
  (`PrimitiveComponent.SetMaterial` _returnvalue_2 0 "/Game/Atlatec/Material/Common/M_SidewalkDev-Master_custom_Roof.M_SidewalkDev-Master_custom_Roof")
  (bind (_arrayindex _arrayelement) (`/Engine/EditorBlueprintResources/StandardMacros.ReverseForEachLoop` _triangulatedindices)
    (:`LoopBody`
      (`KismetArrayLibrary.Array_Add` (`local.Points2D_Reversed`) _arrayelement))
    (:`Completed`
      (bind (_arrayindex_2 _arrayelement_2) (`/Engine/EditorBlueprintResources/StandardMacros.ReverseForEachLoop` _vertices)
        (:`LoopBody`
          (`KismetArrayLibrary.Array_Add` (`local.Vertices_Reversed`) _arrayelement_2))
        (:`Completed`
          (`ProceduralMeshComponent.CreateMeshSection_LinearColor` :`self` _returnvalue_2 :`SectionIndex` 1 :`Vertices` _vertices :`Triangles` (`local.Points2D_Reversed`))
          (`PrimitiveComponent.SetMaterial` _returnvalue_2 1 "/Game/Atlatec/Material/Common/M_SidewalkDev-Master_custom_Roof.M_SidewalkDev-Master_custom_Roof")
          (`ActorComponent.K2_DestroyComponent` _returnvalue)
          (return _returnvalue_2))))))

(fn `UserConstructionScript`)