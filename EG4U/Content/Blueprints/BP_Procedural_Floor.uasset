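; Procedural building floor that lines a spline footprint with facade meshes, rebuilt in the construction script when LiveUpdate is on.
; GenerateFloor tiles each straight segment with instanced base and variation meshes, stretched to fit and alternated by frequency.
; Optional flattened window backdrops draw from ten instance components semi-randomly, and all components support semantic custom-depth stencils.
; Helpers set the footprint, report floor height and clear instances; strip-packing runs, but its output is unused.
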(fn `Calculate number of meshes`
  (params (MeshLength :type "Float (double-precision)") (TotalDistance :type "Float (double-precision)"))
  (returns (Scale :type "Float (double-precision)") (`Number of Meshes` :type Integer))
  (bind _returnvalue (`KismetMathLibrary.FTrunc` (/ TotalDistance MeshLength)))
  (bind _returnvalue_2 (* _returnvalue MeshLength))
  (if (or (== _returnvalue_2 0.0) (== TotalDistance 0.0))
    (return (/ TotalDistance MeshLength) 0)
    (else
      (return (/ TotalDistance _returnvalue_2) (- _returnvalue 1)))))

(fn `CalculateScale`
  (params (SplineLength :type "Float (double-precision)") (MeshSize :type "Float (double-precision)"))
  (returns (Scale :type "Float (double-precision)") (Parts :type Integer))
  (bind (_remainder _returnvalue) (`KismetMathLibrary.FMod` SplineLength MeshSize))
  (bind _returnvalue_2 (!= _returnvalue 0))
  (return (select `bool` _returnvalue_2 :`false` (/ _remainder MeshSize) :`true` (/ SplineLength MeshSize)) (select `bool` _returnvalue_2 :`true` _returnvalue)))

(fn `ConfigureAssets`
  (`KismetArrayLibrary.Array_Clear` (`QuickStripPacking.items_in` (`self.QuickStripPacking`)))
  (for (_array_element _array_index) (`self.FacadePieces`)
    (`KismetArrayLibrary.Array_Add` (`QuickStripPacking.items_in` (`self.QuickStripPacking`)) (make `QuickStripPacking_Item` _array_index (* 2 (.x (`.BoxExtent` (`KismetMathLibrary.BreakBoxSphereBounds` (`StaticMesh.GetBounds` _array_element)))))))))

(fn `GenerateFloor`
  (locals (Frequ :type Integer) (`Corner Rotation` :type "Float (double-precision)") (`Corner Rotation Offset` :type "Float (double-precision)") (CornerOffset :type "Vector Structure"))
  (bind _facade_material (`self.Facade_Material`))
  (bind _ism_variance (`self.ISM_Variance`))
  (bind (_base_bounds_x _base_bounds_y) (`KismetMathLibrary.BreakVector` (`self.Base Bounds`)))
  (bind (_backdropmodifiedextents_x _backdropmodifiedextents_y _backdropmodifiedextents_z) (`KismetMathLibrary.BreakVector` (`self.BackDropModifiedExtents`)))
  (bind _backdropbounds_x (`KismetMathLibrary.BreakVector` (`self.BackDropBounds`)))
  (bind _backdropbounds_x_2 (`KismetMathLibrary.BreakVector` (`self.BackDropBounds`)))
  (bind _backdropbounds_x_3 (`KismetMathLibrary.BreakVector` (`self.BackDropBounds`)))
  (bind (_backdropmodifiedextents_x_2 _backdropmodifiedextents_y_2 _backdropmodifiedextents_z_2) (`KismetMathLibrary.BreakVector` (`self.BackDropModifiedExtents`)))
  (bind _backdropmodifiedextents_x_3 (`KismetMathLibrary.BreakVector` (`self.BackDropModifiedExtents`)))
  (bind _backdropmodifiedextents_x_4 (`KismetMathLibrary.BreakVector` (`self.BackDropModifiedExtents`)))
  (bind _shape (`self.Shape`))
  (bind _backdropmesh (`self.BackDropMesh`))
  (bind _base_bounds_x_2 (`KismetMathLibrary.BreakVector` (`self.Base Bounds`)))
  (bind _variation_bounds_x (`KismetMathLibrary.BreakVector` (`self.Variation Bounds`)))
  (bind _finaltransform (`self.FinalTransform`))
  (bind _shape_2 (`self.Shape`))
  (bind (_properties_basemesh _properties_basetransform _properties_variationfrequency _properties_variationmesh) (break `/EG4U/Data/LevelProperties` (`self.Properties`)))
  (bind _ism_base (`self.ISM_Base`))
  (bind _base_bounds_x_3 (`KismetMathLibrary.BreakVector` (`self.Base Bounds`)))
  (bind _base_bounds_x_4 (`KismetMathLibrary.BreakVector` (`self.Base Bounds`)))
  (bind _finaltransform_2 (`self.FinalTransform`))
  (bind _shape_3 (`self.Shape`))
  (bind _base_bounds_x_5 (`KismetMathLibrary.BreakVector` (`self.Base Bounds`)))
  (bind _base_bounds_x_6 (`KismetMathLibrary.BreakVector` (`self.Base Bounds`)))
  (bind _shape_4 (`self.Shape`))
  (bind (_properties_basemesh_2 _properties_basetransform_2 _properties_variationfrequency_2) (break `/EG4U/Data/LevelProperties` (`self.Properties`)))
  (bind (_returnvalue_origin _returnvalue_boxextent) (`KismetMathLibrary.BreakBoxSphereBounds` (`StaticMesh.GetBounds` _properties_basemesh)))
  (bind (_returnvalue_x _returnvalue_y _returnvalue_z) (`KismetMathLibrary.BreakVector` (/ (`self.Base Bounds`) (`self.BackDropBounds`))))
  (bind _location (`SplineComponent.GetLocationAndTangentAtSplinePoint` _shape_4 0 "Local"))
  (bind _location_2 (`SplineComponent.GetLocationAndTangentAtSplinePoint` _shape_3 0 "Local"))
  (bind _returnvalue (`StaticMesh.GetMaterial` _properties_variationmesh 0))
  (bind _returnvalue_2 (`StaticMesh.GetMaterial` _properties_basemesh 0))
  (bind (_returnvalue_origin_2 _returnvalue_boxextent_2) (`KismetMathLibrary.BreakBoxSphereBounds` (`StaticMesh.GetBounds` _backdropmesh)))
  (bind (_returnvalue_origin_3 _returnvalue_boxextent_3) (`KismetMathLibrary.BreakBoxSphereBounds` (`StaticMesh.GetBounds` _properties_variationmesh)))
  (bind _returnvalue_3 (* _backdropbounds_x_3 _backdropmodifiedextents_x_4))
  ;[1 1 1] Properties
  (`|ExecutionSequence`
    (:`then_0`
      (if (`self.WindowBackdrop`)
        ;[1 1 1] Configure Window Backdrops
        (`|ExecutionSequence`
          (:`then_0`
            (bind _returnvalue_4 (`AddComponent|NODE_AddInstancedStaticMeshComponent-15`))
            (bind _output_get (set `self.ISM_BackDrop_09` _returnvalue_4))
            (`KismetArrayLibrary.Array_Add` (`self.ISM_Refs`) _output_get)
            (`StaticMeshComponent.SetStaticMesh` _returnvalue_4 null)
            (`PrimitiveComponent.SetRenderCustomDepth` _returnvalue_4 (`self.Stencil`))
            (`PrimitiveComponent.SetCustomDepthStencilValue` _returnvalue_4 (`self.Semantic Index`)))
          (:`then_1`
            (bind _returnvalue_5 (`AddComponent|NODE_AddInstancedStaticMeshComponent-14`))
            (bind _output_get_2 (set `self.ISM_BackDrop_08` _returnvalue_5))
            (`KismetArrayLibrary.Array_Add` (`self.ISM_Refs`) _output_get_2)
            (`StaticMeshComponent.SetStaticMesh` _returnvalue_5 null)
            (`PrimitiveComponent.SetRenderCustomDepth` _returnvalue_5 (`self.Stencil`))
            (`PrimitiveComponent.SetCustomDepthStencilValue` _returnvalue_5 (`self.Semantic Index`)))
          (:`then_2`
            (bind _returnvalue_6 (`AddComponent|NODE_AddInstancedStaticMeshComponent-13`))
            (bind _output_get_3 (set `self.ISM_BackDrop_07` _returnvalue_6))
            (`KismetArrayLibrary.Array_Add` (`self.ISM_Refs`) _output_get_3)
            (`StaticMeshComponent.SetStaticMesh` _returnvalue_6 null)
            (`PrimitiveComponent.SetRenderCustomDepth` _returnvalue_6 (`self.Stencil`))
            (`PrimitiveComponent.SetCustomDepthStencilValue` _returnvalue_6 (`self.Semantic Index`)))
          (:`then_3`
            (bind _returnvalue_7 (`AddComponent|NODE_AddInstancedStaticMeshComponent-12`))
            (bind _output_get_4 (set `self.ISM_BackDrop_06` _returnvalue_7))
            (`KismetArrayLibrary.Array_Add` (`self.ISM_Refs`) _output_get_4)
            (`StaticMeshComponent.SetStaticMesh` _returnvalue_7 null)
            (`PrimitiveComponent.SetRenderCustomDepth` _returnvalue_7 (`self.Stencil`))
            (`PrimitiveComponent.SetCustomDepthStencilValue` _returnvalue_7 (`self.Semantic Index`)))
          (:`then_4`
            (bind _returnvalue_8 (`AddComponent|NODE_AddInstancedStaticMeshComponent-11`))
            (bind _output_get_5 (set `self.ISM_BackDrop_05` _returnvalue_8))
            (`KismetArrayLibrary.Array_Add` (`self.ISM_Refs`) _output_get_5)
            (`StaticMeshComponent.SetStaticMesh` _returnvalue_8 null)
            (`PrimitiveComponent.SetRenderCustomDepth` _returnvalue_8 (`self.Stencil`))
            (`PrimitiveComponent.SetCustomDepthStencilValue` _returnvalue_8 (`self.Semantic Index`)))
          (:`then_5`
            (bind _returnvalue_9 (`AddComponent|NODE_AddInstancedStaticMeshComponent-10`))
            (bind _output_get_6 (set `self.ISM_BackDrop_01` _returnvalue_9))
            (`KismetArrayLibrary.Array_Add` (`self.ISM_Refs`) _output_get_6)
            (`StaticMeshComponent.SetStaticMesh` _returnvalue_9 null)
            (`PrimitiveComponent.SetRenderCustomDepth` _returnvalue_9 (`self.Stencil`))
            (`PrimitiveComponent.SetCustomDepthStencilValue` _returnvalue_9 (`self.Semantic Index`)))
          (:`then_6`
            (bind _returnvalue_10 (`AddComponent|NODE_AddInstancedStaticMeshComponent-9`))
            (bind _output_get_7 (set `self.ISM_BackDrop_02` _returnvalue_10))
            (`KismetArrayLibrary.Array_Add` (`self.ISM_Refs`) _output_get_7)
            (`StaticMeshComponent.SetStaticMesh` _returnvalue_10 null)
            (`PrimitiveComponent.SetRenderCustomDepth` _returnvalue_10 (`self.Stencil`))
            (`PrimitiveComponent.SetCustomDepthStencilValue` _returnvalue_10 (`self.Semantic Index`)))
          (:`then_7`
            (bind _returnvalue_11 (`AddComponent|NODE_AddInstancedStaticMeshComponent-8`))
            (bind _output_get_8 (set `self.ISM_BackDrop_03` _returnvalue_11))
            (`KismetArrayLibrary.Array_Add` (`self.ISM_Refs`) _output_get_8)
            (`StaticMeshComponent.SetStaticMesh` _returnvalue_11 null)
            (`PrimitiveComponent.SetRenderCustomDepth` _returnvalue_11 (`self.Stencil`))
            (`PrimitiveComponent.SetCustomDepthStencilValue` _returnvalue_11 (`self.Semantic Index`)))
          (:`then_8`
            (bind _returnvalue_12 (`AddComponent|NODE_AddInstancedStaticMeshComponent-7`))
            (bind _output_get_9 (set `self.ISM_BackDrop_04` _returnvalue_12))
            (`KismetArrayLibrary.Array_Add` (`self.ISM_Refs`) _output_get_9)
            (`StaticMeshComponent.SetStaticMesh` _returnvalue_12 null)
            (`PrimitiveComponent.SetRenderCustomDepth` _returnvalue_12 (`self.Stencil`))
            (`PrimitiveComponent.SetCustomDepthStencilValue` _returnvalue_12 (`self.Semantic Index`)))
          (:`then_9`
            (bind _returnvalue_13 (`AddComponent|NODE_AddInstancedStaticMeshComponent-6`))
            (bind _output_get_10 (set `self.ISM_BackDrop_Base` _returnvalue_13))
            (`KismetArrayLibrary.Array_Add` (`self.ISM_Refs`) _output_get_10)
            (`StaticMeshComponent.SetStaticMesh` _returnvalue_13 _backdropmesh)
            (`PrimitiveComponent.SetRenderCustomDepth` _returnvalue_13 (`self.Stencil`))
            (`PrimitiveComponent.SetCustomDepthStencilValue` _returnvalue_13 (`self.Semantic Index`))
            (set `self.BackDropBounds` _returnvalue_boxextent_2)))))
    (:`then_1`
      ;[0.2 0.2 1] Mesh Extent Calculations
      (bind _returnvalue_14 (`AddComponent|NODE_AddInstancedStaticMeshComponent-0`))
      (bind _output_get_11 (set `self.ISM_Base` _returnvalue_14))
      (`KismetArrayLibrary.Array_Add` (`self.ISM_Refs`) _output_get_11)
      (`StaticMeshComponent.SetStaticMesh` _ism_base _properties_basemesh)
      (`PrimitiveComponent.SetMaterial` _ism_base 0 (select `bool` (== _returnvalue_2 "/EG4U/Mesh/Facades/Material_Instances/M_FACADE_Vertex_Inst01.M_FACADE_Vertex_Inst01") :`false` _returnvalue_2 :`true` _facade_material))
      (`PrimitiveComponent.SetRenderCustomDepth` _ism_base (`self.Stencil`))
      (`PrimitiveComponent.SetCustomDepthStencilValue` _ism_base (`self.Semantic Index`))
      (set `self.Base Bounds` _returnvalue_boxextent))
    (:`then_2`
      (bind _returnvalue_15 (`AddComponent|NODE_AddInstancedStaticMeshComponent-2`))
      (bind _output_get_12 (set `self.ISM_Variance` _returnvalue_15))
      (`KismetArrayLibrary.Array_Add` (`self.ISM_Refs`) _output_get_12)
      (`StaticMeshComponent.SetStaticMesh` _ism_variance _properties_variationmesh)
      (`PrimitiveComponent.SetMaterial` _ism_variance 0 (select `bool` (== _returnvalue "/EG4U/Mesh/Facades/Material_Instances/M_FACADE_Vertex_Inst01.M_FACADE_Vertex_Inst01") :`false` _returnvalue :`true` _facade_material))
      (`PrimitiveComponent.SetRenderCustomDepth` _ism_variance (`self.Stencil`))
      (`PrimitiveComponent.SetCustomDepthStencilValue` _ism_variance (`self.Semantic Index`))
      (set `self.Variation Bounds` _returnvalue_boxextent_3))
    (:`then_3`
      ;[1 0.25 0] Bounding Modifications
      (set `self.BaseFractionVariance` (/ _base_bounds_x_2 _variation_bounds_x))
      (set `self.BackDropModifiedExtents` (`KismetMathLibrary.MakeVector` _returnvalue_x 1.0 _returnvalue_z)))
    (:`then_4`
      ;[1 1 1] Facade
      (`|ExecutionSequence`
        (:`then_0`
          (for _index (range (+ (- (`SplineComponent.GetNumberOfSplinePoints` (`self.Shape`)) 2) 1))
            ;[1 0 0] Straight Middle Segments
            (set `local.Frequ` _properties_variationfrequency_2)
            (set `local.Corner Rotation Offset` 0.0)
            (bind _location_3 (`SplineComponent.GetLocationAndTangentAtSplinePoint` _shape_2 (+ _index 1) "Local"))
            (bind _location_4 (`SplineComponent.GetLocationAndTangentAtSplinePoint` _shape_2 _index "Local"))
            (bind (_scale _number_of_meshes) (`self.Calculate number of meshes` (* 2 _base_bounds_x_3) (`KismetMathLibrary.VSize` (- _location_3 _location_4))))
            (for _index_2 (range (+ _number_of_meshes 1))
              (bind _returnvalue_16 (`KismetMathLibrary.FindLookAtRotation` _location_4 _location_3))
              (set `self.FinalTransform` _returnvalue_16)
              (if (!= (mod _index_2 (`local.Frequ`)) 0)
                (bind _returnvalue_17 (`KismetMathLibrary.TransformLocation` (`KismetMathLibrary.MakeTransform` (+ (* (* (`KismetMathLibrary.Conv_RotatorToVector` _returnvalue_16) _index_2) (* _scale (* 2 _base_bounds_x_4))) _location_4) _returnvalue_16) (0.0 0.0 0.0)))
                (`InstancedStaticMeshComponent.AddInstance` (`self.ISM_Base`) (`KismetMathLibrary.MakeTransform` _returnvalue_17 _finaltransform (`KismetMathLibrary.MakeVector` _scale 1.0 1.0)))
                (else
                  (`InstancedStaticMeshComponent.AddInstance` (`self.ISM_Variance`) (`KismetMathLibrary.MakeTransform` _returnvalue_17 _finaltransform (`KismetMathLibrary.MakeVector` (* _scale (`self.BaseFractionVariance`)) 1.0 1.0)))))))
          ;[1 0 0] Connect Last and First Point
          (if (`self.Closed`)
            (bind _location_5 (`SplineComponent.GetLocationAndTangentAtSplinePoint` _shape_3 _index "Local"))
            (bind (_scale_2 _number_of_meshes_2) (`self.Calculate number of meshes` (* 2 _base_bounds_x_5) (`KismetMathLibrary.VSize` (- _location_2 _location_5))))
            (for _index_3 (range (+ _number_of_meshes_2 1))
              (bind _returnvalue_18 (`KismetMathLibrary.FindLookAtRotation` _location_5 _location_2))
              (set `self.FinalTransform` _returnvalue_18)
              (if (== (mod _index_3 (`local.Frequ`)) 0)
                (bind _returnvalue_19 (+ (* (* (`KismetMathLibrary.Conv_RotatorToVector` _returnvalue_18) _index_3) (* _scale_2 (* 2 _base_bounds_x_6))) _location_5))
                (`InstancedStaticMeshComponent.AddInstance` (`self.ISM_Base`) (`KismetMathLibrary.MakeTransform` _returnvalue_19 _finaltransform_2 (`KismetMathLibrary.MakeVector` _scale_2 1.0 1.0)))
                (else
                  (`InstancedStaticMeshComponent.AddInstance` (`self.ISM_Variance`) (`KismetMathLibrary.MakeTransform` _returnvalue_19 _finaltransform_2 (`KismetMathLibrary.MakeVector` (* _scale_2 (`self.BaseFractionVariance`)) 1.0 1.0))))))))
        (:`then_1`
          ;[1 1 1] Inner Windows
          (if (`self.WindowBackdrop`)
            (for _index_4 (range (+ (- (`SplineComponent.GetNumberOfSplinePoints` (`self.Shape`)) 2) 1))
              ;[1 1 0] Straight Middle Segments
              (set `local.Corner Rotation Offset` 0.0)
              (`self.ConfigureAssets`)
              (bind _location_6 (`SplineComponent.GetLocationAndTangentAtSplinePoint` _shape (+ _index_4 1) "Local"))
              (bind _location_7 (`SplineComponent.GetLocationAndTangentAtSplinePoint` _shape _index_4 "Local"))
              (bind _returnvalue_20 (`KismetMathLibrary.VSize` (- _location_6 _location_7)))
              (`QuickStripPacking.QuickStripPackRuntime` (`self.QuickStripPacking`) _returnvalue_20)
              (bind (_scale_3 _number_of_meshes_3) (`self.Calculate number of meshes` (* 2 _returnvalue_3) _returnvalue_20))
              (if (> _returnvalue_20 _returnvalue_3)
                (for _index_5 (range (+ _number_of_meshes_3 1))
                  (bind _returnvalue_21 (`KismetMathLibrary.FindLookAtRotation` _location_7 _location_6))
                  (set `self.FinalTransform` _returnvalue_21)
                  (bind _returnvalue_22 (+ (* (* (`KismetMathLibrary.Conv_RotatorToVector` _returnvalue_21) _index_5) (* _scale_3 (* 2 _returnvalue_3))) _location_7))
                  (`InstancedStaticMeshComponent.AddInstance` (select `int` (`KismetMathLibrary.Clamp` (mod (`KismetMathLibrary.FTrunc` (`KismetMathLibrary.Abs` (+ (.x _returnvalue_22) (.y _returnvalue_22) (.z _returnvalue_22)))) (`KismetMathLibrary.RandomIntegerInRange` 1 9)) 0 9) :`0` (`self.ISM_BackDrop_Base`) :`1` (`self.ISM_BackDrop_01`) :`2` (`self.ISM_BackDrop_02`) :`3` (`self.ISM_BackDrop_03`) :`4` (`self.ISM_BackDrop_04`) :`5` (`self.ISM_BackDrop_05`) :`6` (`self.ISM_BackDrop_06`) :`7` (`self.ISM_BackDrop_07`) :`8` (`self.ISM_BackDrop_08`) :`9` (`self.ISM_BackDrop_09`)) (`KismetMathLibrary.MakeTransform` (`KismetMathLibrary.TransformLocation` (`KismetMathLibrary.MakeTransform` _returnvalue_22 _returnvalue_21 (1.0 1.0 1.0)) (`KismetMathLibrary.MakeVector` 0.0 (* _base_bounds_y -1.2))) (`self.FinalTransform`) (`KismetMathLibrary.MakeVector` (* _scale_3 _backdropmodifiedextents_x_3) 0.01 _backdropmodifiedextents_z_2))))))
            ;[1 1 0] Connect Last and First Point
            (if (`self.Closed`)
              (bind _location_8 (`SplineComponent.GetLocationAndTangentAtSplinePoint` _shape_4 _index_4 "Local"))
              (bind _returnvalue_23 (`KismetMathLibrary.VSize` (- _location _location_8)))
              (bind (_scale_4 _number_of_meshes_4) (`self.Calculate number of meshes` (* 2 _backdropbounds_x_2) _returnvalue_23))
              (if (> _returnvalue_23 _backdropbounds_x_2)
                (for _index_6 (range (+ _number_of_meshes_4 1))
                  (bind _returnvalue_24 (`KismetMathLibrary.FindLookAtRotation` _location_8 _location))
                  (set `self.FinalTransform` _returnvalue_24)
                  (`InstancedStaticMeshComponent.AddInstance` (`self.ISM_BackDrop_Base`) (`KismetMathLibrary.MakeTransform` (+ (* (* (`KismetMathLibrary.Conv_RotatorToVector` _returnvalue_24) _index_6) (* _scale_4 (* 2 _backdropbounds_x))) _location_8) (`self.FinalTransform`) (`KismetMathLibrary.MakeVector` _scale_4 0.01 _backdropmodifiedextents_z))))))))))
    (:`then_5`
      ;[1 1 1] Linear Tangents
      (for _index_7 (range (`SplineComponent.GetNumberOfSplinePoints` (`self.Shape`)))
        (`SplineComponent.SetSplinePointType` (`self.Shape`) _index_7 "Linear" true)))))

(fn `GetFloorHeight`
  (returns (Height :type "Float (double-precision)"))
  (bind (_properties_basemesh _properties_basetransform _properties_variationfrequency _properties_variationmesh) (break `/EG4U/Data/LevelProperties` (`self.Properties`)))
  (return (* 2 (`KismetMathLibrary.FMax` (.z (`.BoxExtent` (`KismetMathLibrary.BreakBoxSphereBounds` (`StaticMesh.GetBounds` _properties_basemesh)))) (.z (`.BoxExtent` (`KismetMathLibrary.BreakBoxSphereBounds` (`StaticMesh.GetBounds` _properties_variationmesh))))))))

(fn `RemoveFloor`
  (bind _ism_refs (`self.ISM_Refs`))
  (for _array_element _ism_refs
    (`InstancedStaticMeshComponent.ClearInstances` _array_element)
    (`ActorComponent.K2_DestroyComponent` _array_element))
  (`KismetArrayLibrary.Array_Clear` _ism_refs))

(fn `SetFootprint`
  (params (Points :type "Array of Vector Structure") (Height :type "Float (double-precision)") (Reverse :type Boolean))
  (bind _shape (`self.Shape`))
  (if Reverse
    (for _array_element Points
      (`KismetArrayLibrary.Array_Add` (`self.BuildingFootPrint`) (`KismetMathLibrary.MakeVector` (.x _array_element) (.y _array_element) Height)))
    (`SplineComponent.SetSplinePoints` _shape (`self.BuildingFootPrint`) "Local" false :!label _label)
    (for _index (range (`SplineComponent.GetNumberOfSplinePoints` _shape))
      (`SplineComponent.SetSplinePointType` (`self.Shape`) _index "Linear" true))
    (set `self.Closed` true)
    (else
      (bind (_arrayindex _arrayelement) (`/Engine/EditorBlueprintResources/StandardMacros.ReverseForEachLoop` Points)
        (:`LoopBody`
          (`KismetArrayLibrary.Array_Add` (`self.BuildingFootPrint`) (`KismetMathLibrary.MakeVector` (.x _arrayelement) (.y _arrayelement) Height)))
        (:`Completed`
          (goto _label))))))

(fn `UserConstructionScript`
  (`SplineComponent.SetClosedLoop` (`self.Shape`) (`self.Closed`) true)
  (if (`self.LiveUpdate`)
    (`self.GenerateFloor`)))