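; BP_CopyPoints is a utility Blueprint that copies and reverses spline points between actors' spline components.
; CopyPoints appends the SourceActor spline's world-space point locations to a shared Points array, without clearing it, then sets them on the TargetActor's spline.
; ReversePoints clears that array, refills it from the target spline, then rebuilds that spline in reverse order.
; Only locations are read, and no event or construction logic calls either function.
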(fn `CopyPoints`
  (locals (points :type "Array of Vector Structure"))
  (bind _returnvalue (`self.GetComponentByClass` (`self.Target Actor`) "/Script/Engine.SplineComponent"))
  (bind _returnvalue_2 (`self.GetComponentByClass` (`self.Source Actor`) "/Script/Engine.SplineComponent"))
  (if (and (`KismetSystemLibrary.IsValid` _returnvalue_2) (`KismetSystemLibrary.IsValid` _returnvalue))
    (for _index (range (`SplineComponent.GetNumberOfSplinePoints` _returnvalue_2))
      (`KismetArrayLibrary.Array_Add` (`local.points`) (`SplineComponent.GetLocationAtSplinePoint` _returnvalue_2 _index "World")))
    (`SplineComponent.SetSplinePoints` _returnvalue (`local.points`) "World" true)))

(fn `ReversePoints`
  (locals (points :type "Array of Vector Structure"))
  (bind _returnvalue (`self.GetComponentByClass` (`self.Target Actor`) "/Script/Engine.SplineComponent"))
  (`KismetArrayLibrary.Array_Clear` (`local.points`))
  (for _index (range (`SplineComponent.GetNumberOfSplinePoints` _returnvalue))
    (`KismetArrayLibrary.Array_Add` (`local.points`) (`SplineComponent.GetLocationAtSplinePoint` _returnvalue _index "World")))
  (`SplineComponent.ClearSplinePoints` _returnvalue true)
  (bind (_arrayindex _arrayelement) (`/Engine/EditorBlueprintResources/StandardMacros.ReverseForEachLoop` (`local.points`))
    (:`LoopBody`
      (`SplineComponent.AddSplinePoint` _returnvalue _arrayelement "World" true))))

(fn `UserConstructionScript`)