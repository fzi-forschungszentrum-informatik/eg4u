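; Generator actor that builds buildings and roads from OpenStreetMap data held in a StreetMap, with functions to clear each.
; Building ways get their winding normalised by signed area, then become attached BP_OSM_Facade spline actors filled with seeded-random facade meshes through shared instanced mesh components.
; Ways with the chosen attribute become procedural mesh sections built by OSMRoadNetwork.CreateRoadMesh.
; Lane parsing, mesh saving and debug drawing are left unconnected.
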(fn `3Dto2D`
  (params (In :type "Array of Vector Structure"))
  (returns (Out :type "Array of Vector2D Structure"))
  (locals (result :type "Array of Vector2D Structure"))
  (for _array_element In
    (`KismetArrayLibrary.Array_Add` (`local.result`) (`KismetMathLibrary.MakeVector2D` (.x _array_element) (.y _array_element))))
  (return (`local.result`)))

(fn `DebugTriangle`
  (params (Vec :type "Array of Vector Structure") (Tri :type "Array of Integer"))
  (locals (i :type Integer))
  (bind _vec (`local.Vec`))
  (bind _tri (`local.Tri`))
  (bind _i (`local.i`))
  (bind _output (`|GetArrayItem` _vec (`|GetArrayItem` _tri _i)))
  (bind _output_2 (`|GetArrayItem` _vec (`|GetArrayItem` _tri (+ _i 2))))
  (bind _output_3 (`|GetArrayItem` _vec (`|GetArrayItem` _tri (+ _i 1))))
  (while (< (`local.i`) (- (`KismetArrayLibrary.Array_Length` Tri) 2))
    (`KismetSystemLibrary.DrawDebugLine` _output _output_3 (struct :`G` 1.0 :`A` 1.0) 255.0 2.0)
    (`KismetSystemLibrary.DrawDebugLine` _output_3 _output_2 (struct :`G` 1.0 :`A` 1.0) 255.0 2.0)
    (`KismetSystemLibrary.DrawDebugLine` _output_2 _output (struct :`G` 1.0 :`A` 1.0) 255.0 2.0)
    (set `local.i` (+ (`local.i`) 3))))

(fn `Generate Buildings`
  (locals (TempVertsPolygon :type "Array of Vector Structure") (Way_Map :type "Map of Integer to Integer") (Node_Map :type "Map of Integer to Integer"))
  (bind _streetmap (`self.StreetMap`))
  (bind _section_index (`self.Section Index`))
  (bind _returnvalue (`self.K2_GetActorLocation` self))
  (bind _returnvalue_2 (`KismetMathLibrary.RandomIntegerInRangeFromStream` 0 (`KismetArrayLibrary.Array_LastIndex` (`self.Facades`)) (`self.Stream`)))
  (`self.Remove Buildings`)
  (for _array_element (`self.Facades`)
    (bind _returnvalue_3 (`AddComponent|NODE_AddInstancedStaticMeshComponent-0`))
    (`KismetArrayLibrary.Array_Add` (`self.ISM`) _returnvalue_3)
    (`StaticMeshComponent.SetStaticMesh` _returnvalue_3 _array_element))
  (`/Engine/EditorBlueprintResources/StandardMacros.IncrementInt` (`self.Seed`)
    (:`  `
      (if (`KismetSystemLibrary.IsValid` _streetmap)
        (bind _returnvalue_4 (`StreetMapComponent.GetRelationIDsOSM` _streetmap))
        (set `local.Way_Map` _returnvalue_4)
        (bind _returnvalue_5 (`StreetMapComponent.GetNodeIDsOSM` _streetmap))
        (set `local.Node_Map` _returnvalue_5)
        (bind _returnvalue_6 (`StreetMapComponent.GetRoadsOSM` _streetmap))
        (`StreetMapComponent.GetCustomNodesOSM` _streetmap)
        (for _array_element_2 _returnvalue_6
          (switch `EStreetMapRoadType` (`.RoadType` (break `StreetMapRoad` _array_element_2))
            (:`Way_Reference`
              (if (`.ReturnValue` (`BlueprintMapLibrary.Map_Find` (`.Attributes` (break `StreetMapRoad` _array_element_2)) "building"))
                (bind _returnvalue_7 (`StreetMapComponent.Area` (`.RoadPoints` (break `StreetMapRoad` _array_element_2))))
                (bind _returnvalue_8 (< _returnvalue_7 0.0))
                (if _returnvalue_8
                  (for _array_element_3 (`.RoadPoints` (break `StreetMapRoad` _array_element_2))
                    (`KismetArrayLibrary.Array_Add` (`local.TempVertsPolygon`) (+ (`KismetMathLibrary.Conv_Vector2DToVector` _array_element_3) _returnvalue)) ; Save points temporary
                  )
                  (bind _returnvalue_9 (`|SpawnActorFromClass` "/Game/DE/ProceduralGeneration/BP_OSM_Facade.BP_OSM_Facade_C" (`KismetMathLibrary.MakeTransform` (0.0 0.0 0.0)) "AlwaysSpawn" "OverrideRootScale" null null :!label _label))
                  (`SplineComponent.SetSplinePoints` (`/Game/DE/ProceduralGeneration/BP_OSM_Facade.Shape` _returnvalue_9) (select `bool` _returnvalue_8 :`false` (`local.TempVertsPolygon`) :`true` (`local.TempVertsPolygon`)) "Local" true)
                  (set `/Game/DE/ProceduralGeneration/BP_OSM_Facade.MakeRoof` (`self.Make Roof`) _returnvalue_9)
                  (set `/Game/DE/ProceduralGeneration/BP_OSM_Facade.Section Index` (`self.Section Index`) _returnvalue_9)
                  (`/Game/DE/ProceduralGeneration/BP_OSM_Facade.Generate Floor` _returnvalue_9 (`|GetArrayItem` (`self.ISM`) _returnvalue_2) (`|GetArrayItem` (`self.Facades`) _returnvalue_2))
                  (`KismetArrayLibrary.Array_Add` (`self.Buildings`) _returnvalue_9)
                  (`KismetArrayLibrary.Array_Clear` (`local.TempVertsPolygon`))
                  (`KismetArrayLibrary.Array_Clear` (`local.TempVertsPolygon`))
                  (`self.K2_AttachToActor` _returnvalue_9 self "None" "KeepWorld" "KeepWorld" "KeepRelative" true)
                  (`/Engine/EditorBlueprintResources/StandardMacros.IncrementInt` _section_index
                    (:`  `
                      (`/Engine/EditorBlueprintResources/StandardMacros.IncrementInt` _section_index)))
                  (else
                    (bind (_arrayindex _arrayelement) (`/Engine/EditorBlueprintResources/StandardMacros.ReverseForEachLoop` (`.RoadPoints` (break `StreetMapRoad` _array_element_2)))
                      (:`LoopBody`
                        (`KismetArrayLibrary.Array_Add` (`local.TempVertsPolygon`) (+ _returnvalue (`KismetMathLibrary.Conv_Vector2DToVector` _arrayelement))) ; Save points temporary
                      )
                      (:`Completed`
                        (goto _label)))))))))
        (`/Engine/EditorBlueprintResources/StandardMacros.IncrementInt` (`self.Seed`))
        (else
          (`KismetSystemLibrary.PrintString` "Error: file not valid"))))))

(fn `Generate Roads`
  (locals (current_tri :type Integer))
  (bind _streetmap (`self.StreetMap`))
  (bind _streetmap_2 (`self.StreetMap`))
  (`StreetMapComponent.GetStreetMap` _streetmap)
  (if (and (`KismetSystemLibrary.IsValid` _streetmap) (`KismetSystemLibrary.IsValid` _streetmap))
    (bind _returnvalue (`StreetMapComponent.GetRelationIDsOSM` _streetmap_2))
    (set `self.Way_Map` _returnvalue)
    (bind _returnvalue_2 (`StreetMapComponent.GetNodeIDsOSM` _streetmap_2))
    (set `self.Node_Map` _returnvalue_2)
    (bind _returnvalue_3 (`StreetMapComponent.GetRoadsOSM` _streetmap_2))
    (`StreetMapComponent.GetCustomNodesOSM` _streetmap_2)
    (for (_array_element _array_index) _returnvalue_3
      (switch `EStreetMapRoadType` (`.RoadType` (break `StreetMapRoad` _array_element))
        (:`Way_Reference`
          (bind _returnvalue_4 (`AddComponent|NODE_AddProceduralMeshComponent-5`))
          (if (`.ReturnValue` (`BlueprintMapLibrary.Map_Find` (`.Attributes` (break `StreetMapRoad` _array_element)) (`self.Attribute`)))
            (bind _returnvalue_5 (`OSM_RoadNetwork.CreateRoadMesh` (`self.OSM_RoadNetwork`) (`.RoadPoints` (break `StreetMapRoad` _array_element)) (`.Attributes` (break `StreetMapRoad` _array_element)) 0 (`self.Lane Width`) 500.0 30.0 (`self.Resolution`)))
            (if (== (mod (`KismetArrayLibrary.Array_Length` (`.indices` (break `OSM_Mesh` _returnvalue_5))) 3) 0)
              (`ProceduralMeshComponent.CreateMeshSection_LinearColor` :`self` _returnvalue_4 :`SectionIndex` _array_index :`Vertices` (break `OSM_Mesh` _returnvalue_5) :`Triangles` (`.indices` (break `OSM_Mesh` _returnvalue_5)))
              (`PrimitiveComponent.SetMaterial` _returnvalue_4 _array_index (`self.Material`))
              (`KismetArrayLibrary.Array_Add` (`self.RoadMeshes`) _returnvalue_4))))))))

(fn `Remove Buildings`
  (bind _ism (`self.ISM`))
  (bind _buildings (`self.Buildings`))
  (for _array_element _buildings
    (`self.K2_DestroyActor` _array_element))
  (`KismetArrayLibrary.Array_Clear` _buildings)
  (`KismetSystemLibrary.PrintString` "clean...")
  (for _array_element_2 _ism
    (`InstancedStaticMeshComponent.ClearInstances` _array_element_2)
    (`ActorComponent.K2_DestroyComponent` _array_element_2))
  (`KismetArrayLibrary.Array_Clear` _ism))

(fn `Remove roads`
  (bind _roadmeshes (`self.RoadMeshes`))
  (for _array_element _roadmeshes
    (`ProceduralMeshComponent.ClearAllMeshSections` _array_element)
    (`ActorComponent.K2_DestroyComponent` _array_element))
  (`KismetArrayLibrary.Array_Clear` _roadmeshes)
  (`KismetSystemLibrary.FlushPersistentDebugLines`))

(fn `UserConstructionScript`
  (`KismetMathLibrary.SetRandomStreamSeed` (`self.Stream`) (`self.Seed`)))